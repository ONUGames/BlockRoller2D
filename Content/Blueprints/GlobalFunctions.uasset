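; GlobalFunctions is a shared helper Blueprint for level section selection and save data access.
; It maps difficulty tiers to section lists and picks a random section, attempting to exclude a given one.
; It creates, loads and writes a single GlobalSave slot.
; IsDelayLong reads the First flag from a save slot named after the current level, defaulting to true when none exists.
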(fn GetPackNames
  (return (LocalVariables|GetNewLocalVar_0)))

(fn GetSections
  (params (Difficulty :type E_Difficulties%20Enum :default "NewEnumerator0"))
  (switch Utilities|FlowControl|Switch|SwitchonE_Difficulties Difficulty
    (:NewEnumerator0
      (return (LocalVariables|GetL_SectionsEasy)))
    (:NewEnumerator1
      (return (LocalVariables|GetL_SectionsNormal)))
    (:NewEnumerator2
      (return (LocalVariables|GetL_SectionsHard)))
    (:NewEnumerator3
      (return (LocalVariables|GetL_SectionsExtreme)))
    (:NewEnumerator4
      (return (LocalVariables|GetL_SectionsDemonic)))))

(fn GetRandomSection
  (params (Exept :type BP%20Standart%20Section%20Class%20Reference) (Difficulty :type E_Difficulties%20Enum :default "NewEnumerator0"))
  (bind _sections (CallFunction|GetSections Difficulty))
  (Utilities|Array|RemoveItem _sections Exept)
  (return (Utilities|Array|Get(acopy) _sections (Math|Random|RandomIntegerinRange 0 (- (Utilities|Array|Length _sections) 1)))))

(fn GetGlobalSave
  (bind _returnvalue (SaveGame|DoesSaveGameExist "GlobalSave"))
  (if _returnvalue
    _
    (else
      (bind _returnvalue_2 (SaveGame|CreateSaveGameObject "/Game/Blueprints/BP_GlobalSave.BP_GlobalSave_C"))
      (SaveGame|SaveGametoSlot _returnvalue_2 "GlobalSave")))
  (bind _returnvalue_3 (SaveGame|LoadGamefromSlot "GlobalSave"))
  (return (.AsBP%20Global%20Save (Utilities|Casting|CastToBP_GlobalSave _returnvalue_3))))

(fn SaveGlobal
  (params (SaveGameObject :type Save%20Game%20Object%20Reference))
  (SaveGame|SaveGametoSlot SaveGameObject "GlobalSave"))

(fn IsDelayLong
  (bind _returnvalue (Game|GetCurrentLevelName 0))
  (bind _returnvalue_2 (SaveGame|DoesSaveGameExist _returnvalue))
  (if _returnvalue_2
    (bind _returnvalue_3 (SaveGame|LoadGamefromSlot _returnvalue))
    (return (Variables|/Game/Blueprints/BP_SaveLevel.BP_SaveLevel_C|GetFirst (.AsBP%20Save%20Level (Utilities|Casting|CastToBP_SaveLevel _returnvalue_3))))
    (else
      (return true))))