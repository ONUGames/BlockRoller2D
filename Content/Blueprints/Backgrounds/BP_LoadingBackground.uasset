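; Parallax menu/loading backdrop that stacks Paper2D sprites for the current menu season at stepped depths, built in both the construction script and BeginPlay.
; An intro timeline drives Pos, which shifts each layer vertically in proportion to its index.
; Load stops it and calls AnimMove, whose timeline eases Pos to a vertical preset and slides the actor horizontally to the last played season or infinity mode saved.
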(event Custom|Load
  (Utilities|FlowControl|Sequence
    (:then_0
      (bind _newtrack_0 (Timeline|Timeline_0 Stop)
        (:Update
          (Variables|Default|SetPos _newtrack_0)
          (CallFunction|UpdatePos))))
    (:then_1
      (bind _asbp_global_save (CallFunction|GetGlobalSave))
      (if (Utilities|Enum|Equal(Enum) (Variables|/Game/Blueprints/BP_GlobalSave.BP_GlobalSave_C|GetLast%20Level%20Played _asbp_global_save) "None")
        (CallFunction|AnimMove)
        (elif (Utilities|Enum|Equal(Enum) (.LeftS (Utilities|String|Split (Variables|/Game/Blueprints/BP_GlobalSave.BP_GlobalSave_C|GetLast%20Level%20Played _asbp_global_save) "_")) "infinitymode")
          (CallFunction|AnimMove 1 (+ (CallFunction|GetAmountOfSeasons) 1))
          (else
            (bind (_array_element _array_index) (Utilities|Array|ForEachLoopwithBreak (CallFunction|GetSeasonNames))
              (:LoopBody
                (if (Utilities|Enum|Equal(Enum) _array_element (.LeftS (Utilities|String|Split (Variables|/Game/Blueprints/BP_GlobalSave.BP_GlobalSave_C|GetLast%20Level%20Played _asbp_global_save) "_")))
                  (CallFunction|AnimMove 1 (+ _array_index 1)))))))))))

(event Custom|AnimMove
  (params (Vertical :type Integer) (Horizontal :type Integer))
  (Variables|Default|SetP_HorAnim (.X (Math|Vector|BreakVector (Transformation|GetActorLocation self))))
  (Variables|Default|SetOldPos (Variables|Default|GetPos))
  (switch int Vertical
    (:0
      (Variables|Default|SetNewPos 1.0)
      (bind _newtrack_0 (Timeline|Timeline_1 PlayFromStart)
        (:Update
          (Utilities|FlowControl|Sequence
            (:then_0
              (Variables|Default|SetPos (+ (* (- (Variables|Default|GetNewPos) (Variables|Default|GetOldPos)) _newtrack_0) (Variables|Default|GetOldPos)))
              (CallFunction|UpdatePos))
            (:then_1
              (Transformation|SetActorLocation (Math|Vector|MakeVector (+ (* _newtrack_0 (- (- 2.6e+03 (* (/ (Math|Conversions|ToFloat(Integer) Horizontal) (Math|Conversions|ToFloat(Integer) (+ (CallFunction|GetAmountOfSeasons) 2))) 5.2e+03)) (Variables|Default|GetP_HorAnim))) (Variables|Default|GetP_HorAnim)) -3e+03 0.0) false false))))))
    (:1
      (Variables|Default|SetNewPos 0.5)
      (Timeline|Timeline_1 PlayFromStart))
    (:2
      (Variables|Default|SetNewPos 0.0)
      (Timeline|Timeline_1 PlayFromStart))))

(event EventBeginPlay
  (bind _result (CallFunction|GetMenuSeason))
  (Variables|Default|SetSeason _result)
  (for (_array_element _array_index) (CallFunction|GetParallaxSpritesbySeason (Variables|Default|GetSeason))
    (bind _returnvalue (AddComponent|AddPaperSpriteComponent false (Math|Transform|MakeTransform (Math|Vector|MakeVector 0.0 (+ (* _array_index 7e+02) -2e+03) 0.0))))
    (Utilities|Array|Add (Variables|Default|GetSprites) _returnvalue)
    (Rendering|Components|Sprite|SetSprite _returnvalue _array_element))
  (Transformation|SetActorLocation "0.000000,-4000.000000, 0" false false)
  (bind _newtrack_0 (Timeline|Timeline_0 Play)
    (:Update
      (Variables|Default|SetPos _newtrack_0)
      (CallFunction|UpdatePos))))

(fn ConstructionScript
  (bind _result (CallFunction|GetMenuSeason))
  (Variables|Default|SetSeason _result)
  (for (_array_element _array_index) (CallFunction|GetParallaxSpritesbySeason (Variables|Default|GetSeason))
    (bind _returnvalue (AddComponent|AddPaperSpriteComponent false (Math|Transform|MakeTransform (Math|Vector|MakeVector 0.0 (+ (* _array_index 7e+02) -2e+03) 0.0))))
    (Utilities|Array|Add (Variables|Default|GetSprites) _returnvalue)
    (Rendering|Components|Sprite|SetSprite _returnvalue _array_element))
  (Transformation|SetActorLocation "0.000000,-4000.000000, 0" false false))

(fn Move
  (params (Koef :type Float%20%28single-precision%29) (Sprite :type Paper%20Sprite%20Component%20Object%20Reference))
  (Transformation|SetRelativeLocation Sprite (Math|Vector|MakeVector 0.0 (.Y (Math|Vector|BreakVector (Variables|/Script/Engine.SceneComponent|GetRelativeLocation Sprite))) (* (* (Variables|Default|GetPos) -8e+02) Koef)) false false))

(fn UpdatePos
  (for (_array_element _array_index) (Variables|Default|GetSprites)
    (CallFunction|Move (* _array_index 0.3) _array_element)))