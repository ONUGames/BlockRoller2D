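; Parallax menu background of clouds, birds, rocks and pines that follows the main character's side-view camera vertically.
; On BeginPlay it caches the character and start location, and parses the number after the underscore in the level name.
; Each Tick places it horizontally by that number and at camera height.
; Move then offsets each sprite layer by height change times a per-layer coefficient, also applied in the Construction Script.
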(event Custom|UpdatePos
  (CallFunction|Move 0.3 (Variables|Default|Getclouds_1_Sprite))
  (CallFunction|Move 0.4 (Variables|Default|Getclouds_2_Sprite))
  (CallFunction|Move 0.5 (Variables|Default|Getclouds_3_Sprite))
  (CallFunction|Move 0.6 (Variables|Default|Getclouds_3_Sprite))
  (CallFunction|Move 0.7 (Variables|Default|Getbirds_Sprite))
  (CallFunction|Move 0.9 (Variables|Default|Getrocks_2_Sprite))
  (CallFunction|Move 1.0 (Variables|Default|Getrocks_2_Sprite))
  (CallFunction|Move 1.2 (Variables|Default|Getrocks_3_Sprite))
  (CallFunction|Move 1.3 (Variables|Default|Getrocks_1_Sprite))
  (CallFunction|Move 1.5 (Variables|Default|Getpines_Sprite)))

(event EventTick
  (params (DeltaSeconds :type Float%20%28single-precision%29))
  (Transformation|SetActorLocation (Math|Vector|MakeVector (- (* (/ (Math|Conversions|ToFloat(Integer) (Variables|Default|GetFromLeft)) 32.0) 5.2e+03) 2.6e+03) -3e+03 (.Z (Math|Vector|BreakVector (Transformation|GetWorldLocation (Variables|/Game/Blueprints/Characters/BP_Character_Main.BP_Character_Main_C|GetSideViewCameraComponent (Variables|Default|GetCharacter)))))) false false)
  (Variables|Default|SetPos (/ (- (.Z (Math|Vector|BreakVector (Transformation|GetActorLocation))) (.Z (Math|Vector|BreakVector (Variables|Default|GetNewVar_0)))) 5e+03))
  (CallFunction|UpdatePos))

(event EventBeginPlay
  (bind _outactors (Actor|GetAllActorsOfClass "/Game/Blueprints/Characters/BP_Character_Main.BP_Character_Main_C"))
  (Variables|Default|SetCharacter (Utilities|Array|Get(acopy) _outactors))
  (Variables|Default|SetNewVar_0 (Transformation|GetActorLocation))
  (bind _returnvalue (Game|GetCurrentLevelName true))
  (Variables|Default|SetFromLeft (Math|Conversions|ToInteger(Byte) (.RightS (Utilities|String|Split _returnvalue "_")))))

(fn ConstructionScript
  (CallFunction|UpdatePos))

(fn Move
  (params (Koef :type Float%20%28single-precision%29) (Sprite :type Paper%20Sprite%20Component%20Object%20Reference))
  (Transformation|SetRelativeLocation Sprite (Math|Vector|MakeVector 0.0 (.Y (Math|Vector|BreakVector (Variables|/Script/Engine.SceneComponent|GetRelativeLocation Sprite))) (* (* (Variables|Default|GetPos) -8e+02) Koef)) false false))