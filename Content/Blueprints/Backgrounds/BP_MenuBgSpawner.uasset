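; BP_MenuBgSpawner places the menu background actor at its own transform, using a fixed stretched scale.
; On BeginPlay it reads MenuBgSetting from the global save to spawn one of four BP_MenuBG variants.
; Setting 0 chooses automatically from the last played level's name prefix (Lake, Mountain, Night Forest, Waterfall), defaulting to the first.
; The Update event destroys the current background, then repeats the selection.
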(event Custom|Update
  (bind _self self)
  (bind _returnvalue (Transformation|GetActorTransform _self))
  (bind (_location _rotation) (Math|Transform|BreakTransform _returnvalue))
  (bind _returnvalue_2 (Math|Transform|MakeTransform _location _rotation "4.000000,1,3.500000"))
  (Utilities|IsValid (Variables|Default|GetCurrent)
    (:Is%20Valid
      (Actor|DestroyActor (Variables|Default|GetCurrent)))
    (:Is%20Not%20Valid
      _))
  (bind _asbp_global_save (CallFunction|GetGlobalSave))
  (switch int (Variables|/Game/Blueprints/BP_GlobalSave.BP_GlobalSave_C|GetMenuBgSetting _asbp_global_save)
    (:0
      (switch string (.LeftS (Utilities|String|Split (Variables|/Game/Blueprints/BP_GlobalSave.BP_GlobalSave_C|GetLast%20Level%20Played _asbp_global_save) "_"))
        (:Default
          (bind _returnvalue_3 (Game|SpawnActorfromClass "/Game/Blueprints/Backgrounds/BP_MenuBG_1.BP_MenuBG_1_C" _returnvalue_2 "Undefined" _self 0 :!label _label))
          (Variables|Default|SetCurrent _returnvalue_3))
        (:Lake
          (goto _label))
        (:Mountain
          (bind _returnvalue_4 (Game|SpawnActorfromClass "/Game/Blueprints/Backgrounds/BP_MenuBG_2.BP_MenuBG_2_C" _returnvalue_2 "Undefined" _self 0 :!label _label_2))
          (Variables|Default|SetCurrent _returnvalue_4))
        (:NightForest
          (bind _returnvalue_5 (Game|SpawnActorfromClass "/Game/Blueprints/Backgrounds/BP_MenuBG_3.BP_MenuBG_3_C" _returnvalue_2 "Undefined" _self 0 :!label _label_3))
          (Variables|Default|SetCurrent _returnvalue_5))
        (:Waterfall
          (bind _returnvalue_6 (Game|SpawnActorfromClass "/Game/Blueprints/Backgrounds/BP_MenuBG_4.BP_MenuBG_4_C" _returnvalue_2 "Undefined" _self 0 :!label _label_4))
          (Variables|Default|SetCurrent _returnvalue_6))))
    (:1
      (goto _label))
    (:2
      (goto _label_2))
    (:3
      (goto _label_3))
    (:4
      (goto _label_4))))

(event EventBeginPlay
  (bind _self self)
  (bind _returnvalue (Transformation|GetActorTransform _self))
  (bind (_location _rotation) (Math|Transform|BreakTransform _returnvalue))
  (bind _returnvalue_2 (Math|Transform|MakeTransform _location _rotation "4.000000,1,3.500000"))
  (bind _asbp_global_save (CallFunction|GetGlobalSave))
  (switch int (Variables|/Game/Blueprints/BP_GlobalSave.BP_GlobalSave_C|GetMenuBgSetting _asbp_global_save)
    (:0
      (switch string (.LeftS (Utilities|String|Split (Variables|/Game/Blueprints/BP_GlobalSave.BP_GlobalSave_C|GetLast%20Level%20Played _asbp_global_save) "_"))
        (:Default
          (bind _returnvalue_3 (Game|SpawnActorfromClass "/Game/Blueprints/Backgrounds/BP_MenuBG_1.BP_MenuBG_1_C" _returnvalue_2 "Undefined" _self 0 :!label _label))
          (Variables|Default|SetCurrent _returnvalue_3))
        (:Lake
          (goto _label))
        (:Mountain
          (bind _returnvalue_4 (Game|SpawnActorfromClass "/Game/Blueprints/Backgrounds/BP_MenuBG_2.BP_MenuBG_2_C" _returnvalue_2 "Undefined" _self 0 :!label _label_2))
          (Variables|Default|SetCurrent _returnvalue_4))
        (:NightForest
          (bind _returnvalue_5 (Game|SpawnActorfromClass "/Game/Blueprints/Backgrounds/BP_MenuBG_3.BP_MenuBG_3_C" _returnvalue_2 "Undefined" _self 0 :!label _label_3))
          (Variables|Default|SetCurrent _returnvalue_5))
        (:Waterfall
          (bind _returnvalue_6 (Game|SpawnActorfromClass "/Game/Blueprints/Backgrounds/BP_MenuBG_4.BP_MenuBG_4_C" _returnvalue_2 "Undefined" _self 0 :!label _label_4))
          (Variables|Default|SetCurrent _returnvalue_6))))
    (:1
      (goto _label))
    (:2
      (goto _label_2))
    (:3
      (goto _label_3))
    (:4
      (goto _label_4))))

(fn ConstructionScript)