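; Layered sprite background actor, apparently for a menu, with clouds, rocks and ground that scroll with parallax.
; MoveVer uses a timeline to blend Pos to a target; UpdatePos then offsets each layer vertically by its own depth coefficient, also applied in the construction script.
; MoveHor uses a second timeline to slide the whole actor along X to an indexed stop, starting from the far positive end set on BeginPlay.
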(event Custom|UpdatePos
  (CallFunction|Move 0.6 (Variables|Default|Getclouds_1_Sprite))
  (CallFunction|Move 0.8 (Variables|Default|Getclouds_2_Sprite))
  (CallFunction|Move 1.0 (Variables|Default|Getrocks_Sprite))
  (CallFunction|Move 1.4 (Variables|Default|Getground_Sprite)))

(event EventMoveVer
  (params (To :type Float%20%28single-precision%29))
  (bind _output_get (Variables|Default|SetNewVar_1 (Variables|Default|GetPos)))
  (bind _newtrack_0 (Timeline|Timeline_0 PlayFromStart)
    (:Update
      (Variables|Default|SetPos (+ (* _newtrack_0 (- To _output_get)) _output_get))
      (CallFunction|UpdatePos))))

(event EventMoveHor
  (params (To :type Integer))
  (bind _output_get (Variables|Default|SetNewVar_2 (.X (Math|Vector|BreakVector (Transformation|GetActorLocation self)))))
  (bind _newtrack_0 (Timeline|Timeline_1 PlayFromStart)
    (:Update
      (Transformation|SetActorLocation (Math|Vector|MakeVector (+ (* _newtrack_0 (- (- (* (/ (Math|Conversions|ToFloat(Integer) (- 6 To)) 6.0) 5.2e+03) 2.6e+03) _output_get)) _output_get) -3e+03 0.0) false false))))

(event EventBeginPlay
  (Transformation|SetActorLocation (Math|Vector|MakeVector (- (* (/ (Math|Conversions|ToFloat(Integer) 32) 32.0) 5.2e+03) 2.6e+03) -3e+03 0.0) false false))

(fn ConstructionScript
  (CallFunction|UpdatePos))

(fn Move
  (params (Koef :type Float%20%28single-precision%29) (Sprite :type Paper%20Sprite%20Component%20Object%20Reference))
  (Transformation|SetRelativeLocation Sprite (Math|Vector|MakeVector 0.0 (.Y (Math|Vector|BreakVector (Variables|/Script/Engine.SceneComponent|GetRelativeLocation Sprite))) (* (* (Variables|Default|GetPos) -8e+02) Koef)) false false))