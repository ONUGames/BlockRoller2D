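; BP_LoadingBg_1 is a layered sprite background, named for a loading screen, with two rock and four cloud layers that shift for a parallax effect.
; UpdatePos passes each sprite to Move with its own coefficient, so rocks travel farther than clouds.
; Move sets relative Z from the Pos variable scaled by that coefficient, keeping Y and zeroing X.
; The construction script calls UpdatePos to apply the current Pos.
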(event Custom|UpdatePos
  (CallFunction|Move 1.0 (Variables|Default|Getrocks_1_Sprite))
  (CallFunction|Move 1.3 (Variables|Default|Getrocks_2_Sprite))
  (CallFunction|Move 0.2 (Variables|Default|Getclouds_1_Sprite))
  (CallFunction|Move 0.4 (Variables|Default|Getclouds_2_Sprite))
  (CallFunction|Move 0.6 (Variables|Default|Getclouds_3_Sprite))
  (CallFunction|Move 0.8 (Variables|Default|Getclouds_4_Sprite)))

(fn ConstructionScript
  (CallFunction|UpdatePos))

(fn Move
  (params (Koef :type Float%20%28single-precision%29) (Sprite :type Paper%20Sprite%20Component%20Object%20Reference))
  (Transformation|SetRelativeLocation Sprite (Math|Vector|MakeVector 0.0 (.Y (Math|Vector|BreakVector (Variables|/Script/Engine.SceneComponent|GetRelativeLocation Sprite))) (* (* (Variables|Default|GetPos) -8e+02) Koef)) false false))