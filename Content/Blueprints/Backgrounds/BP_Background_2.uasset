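; Layered parallax background actor for side-view levels, with clouds, birds, rocks and pines.
; Each tick through a gate, it follows the main character's camera height, takes its X offset from the number in the level name, and shifts sprites vertically by per-layer coefficients.
; Secret chamber events move it to the chamber and close the gate, then restore its start position and reopen the gate on leaving.
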(event Custom|UpdatePos
  (CallFunction|Move 0.3 (Variables|Default|Getclouds_1_Sprite))
  (CallFunction|Move 0.4 (Variables|Default|Getclouds_2_Sprite))
  (CallFunction|Move 0.5 (Variables|Default|Getclouds_3_Sprite))
  (CallFunction|Move 0.6 (Variables|Default|Getclouds_3_Sprite))
  (CallFunction|Move 0.7 (Variables|Default|Getbirds_Sprite))
  (CallFunction|Move 0.9 (Variables|Default|Getrocks_2_Sprite))
  (CallFunction|Move 1.0 (Variables|Default|Getrocks_2_Sprite))
  (CallFunction|Move 1.2 (Variables|Default|Getrocks_3_Sprite))
  (CallFunction|Move 1.3 (Variables|Default|Getrocks_1_Sprite))
  (CallFunction|Move 1.5 (Variables|Default|Getpines_Sprite)))

(event Custom|Event%20Secret%20Chamber_Event_0
  (params (Entered :type Boolean) (Location :type Vector%202D%20Structure))
  (bind (_x _y) (Math|Vector2D|BreakVector2D Location))
  (if Entered
    (Transformation|SetActorLocation (Math|Vector|MakeVector _x -3e+03 _y) false false)
    (Utilities|FlowControl|Gate false) ; enters at Close
    (else
      (Transformation|SetActorLocation (Variables|Default|GetBeginCoords) false false)
      (Utilities|FlowControl|Gate false) ; enters at Open
    )))

(event EventTick
  (params (DeltaSeconds :type Float%20%28single-precision%29))
  (Utilities|FlowControl|Gate false
    (:Exit
      (Transformation|SetActorLocation (Math|Vector|MakeVector (- (* (/ (Math|Conversions|ToFloat(Integer) (Variables|Default|GetFromLeft)) 32.0) 5.2e+03) 2.6e+03) -3e+03 (.Z (Math|Vector|BreakVector (Transformation|GetWorldLocation (Variables|/Game/Blueprints/Characters/BP_Character_Main.BP_Character_Main_C|GetSideViewCameraComponent (Variables|Default|GetCharacter)))))) false false)
      (Variables|Default|SetPos (/ (- (.Z (Math|Vector|BreakVector (Transformation|GetActorLocation))) (.Z (Math|Vector|BreakVector (Variables|Default|GetNewVar_0)))) 5e+03))
      (CallFunction|UpdatePos))))

(event EventBeginPlay
  (bind _returnvalue (Transformation|GetActorLocation))
  (bind _outactors (Actor|GetAllActorsOfClass "/Game/Blueprints/Characters/BP_Character_Main.BP_Character_Main_C"))
  (bind _output_get (Variables|Default|SetCharacter (Utilities|Array|Get(acopy) _outactors)))
  (Variables|Default|SetBeginCoords _returnvalue)
  (Variables|Default|SetNewVar_0 _returnvalue)
  (bind _returnvalue_2 (Game|GetCurrentLevelName true))
  (Variables|Default|SetFromLeft (Math|Conversions|ToInteger(Byte) (.RightS (Utilities|String|Split _returnvalue_2 "_"))))
  (EventDispatchers|AssignEventSecretChamber _output_get (delegate Custom|Event%20Secret%20Chamber_Event_0)))

(fn ConstructionScript
  (CallFunction|UpdatePos))

(fn Move
  (params (Koef :type Float%20%28single-precision%29) (Sprite :type Paper%20Sprite%20Component%20Object%20Reference))
  (Transformation|SetRelativeLocation Sprite (Math|Vector|MakeVector 0.0 (.Y (Math|Vector|BreakVector (Variables|/Script/Engine.SceneComponent|GetRelativeLocation Sprite))) (* (* (Variables|Default|GetPos) -8e+02) Koef)) false false))