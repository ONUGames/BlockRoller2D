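; Infinite parallax background actor that follows the main character's side-view camera vertically.
; The construction script picks a random season and spawns one Paper2D sprite component per parallax sprite of that season, spaced in depth along Y.
; Each tick it snaps to the camera's height, then offsets each sprite against the distance travelled from its start, scaled by layer index, so layers scroll at different rates.
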(event EventTick
  (params (DeltaSeconds :type Float%20%28single-precision%29))
  (Transformation|SetActorLocation (Math|Vector|MakeVector 0.0 -4e+03 (.Z (Math|Vector|BreakVector (Transformation|GetWorldLocation (Variables|/Game/Blueprints/Characters/BP_Character_Main.BP_Character_Main_C|GetSideViewCameraComponent (Variables|Default|GetCharacter)))))) false true)
  (Variables|Default|SetPos (/ (- (.Z (Math|Vector|BreakVector (Transformation|GetActorLocation))) (.Z (Math|Vector|BreakVector (Variables|Default|GetBeginCoords)))) 1e+05))
  (CallFunction|UpdatePos))

(event EventBeginPlay
  (Transformation|SetActorLocation "0,-10000.000000,0.000000" false false)
  (bind _outactors (Actor|GetAllActorsOfClass "/Game/Blueprints/Characters/BP_Character_Main.BP_Character_Main_C"))
  (Variables|Default|SetCharacter (Utilities|Array|Get(acopy) _outactors))
  (Variables|Default|SetBeginCoords (Transformation|GetActorLocation)))

(fn ConstructionScript
  (Variables|Default|SetSeason (Utilities|Enum|ByteToEnumE_Season (Math|Conversions|ToByte(Integer) (Math|Random|RandomIntegerinRange 0 (- (CallFunction|GetAmountOfSeasons) 1)))))
  (for (_array_element _array_index) (CallFunction|GetParallaxSpritesbySeason (Variables|Default|GetSeason))
    (bind _returnvalue (AddComponent|AddPaperSpriteComponent false (Math|Transform|MakeTransform (Math|Vector|MakeVector 0.0 (+ (* _array_index 7e+02) -2e+03) 0.0))))
    (Utilities|Array|Add (Variables|Default|GetSprites) _returnvalue)
    (Rendering|Components|Sprite|SetSprite _returnvalue _array_element)))

(fn Move
  (params (Koef :type Float%20%28single-precision%29) (Sprite :type Paper%20Sprite%20Component%20Object%20Reference))
  (Transformation|SetRelativeLocation Sprite (Math|Vector|MakeVector 0.0 (.Y (Math|Vector|BreakVector (Variables|/Script/Engine.SceneComponent|GetRelativeLocation Sprite))) (* (* (Variables|Default|GetPos) -8e+02) Koef)) false false))

(fn UpdatePos
  (for (_array_element _array_index) (Variables|Default|GetSprites)
    (CallFunction|Move (* _array_index 0.3) _array_element)))