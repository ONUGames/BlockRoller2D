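; Parallax menu background that builds layered Paper2D sprites for the current menu season and scrolls between menu positions.
; Construction places it at the season or infinity mode of the last level played in the global save.
; Horizontal moves slide the whole actor across slots derived from season count, animated by a timeline.
; Vertical moves animate VerPosition, whose OnRep offsets each sprite's height by a layer-index factor.
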(event Custom|MoveVer
  (params (To :type Float%20%28single-precision%29))
  (Variables|Default|SetP_VerAnim (Variables|Default|GetVer%20Position))
  (bind _newtrack_0 (Timeline|Timeline_0 PlayFromStart)
    (:Update
      (Variables|Default|SetVer%20Position (+ (* _newtrack_0 (- To (Variables|Default|GetP_VerAnim))) (Variables|Default|GetP_VerAnim))))))

(event Custom|MoveHor
  (params (To :type Integer))
  (Variables|Default|SetP_HorAnim (.X (Math|Vector|BreakVector (Transformation|GetActorLocation self))))
  (bind _newtrack_0 (Timeline|Timeline_1 PlayFromStart)
    (:Update
      (Transformation|SetActorLocation (Math|Vector|MakeVector (+ (* _newtrack_0 (- (- 2.6e+03 (* (/ (Math|Conversions|ToFloat(Integer) To) (Math|Conversions|ToFloat(Integer) (+ (CallFunction|GetAmountOfSeasons) 2))) 5.2e+03)) (Variables|Default|GetP_HorAnim))) (Variables|Default|GetP_HorAnim)) -3e+03 0.0) false false))))

(fn ConstructionScript
  (Public|Refresh false)
  (bind _asbp_global_save (CallFunction|GetGlobalSave))
  (if (Utilities|Enum|Equal(Enum) (Variables|/Game/Blueprints/BP_GlobalSave.BP_GlobalSave_C|GetLast%20Level%20Played _asbp_global_save) "None")
    (Public|MoveNoAnim)
    (elif (Utilities|Enum|Equal(Enum) (.LeftS (Utilities|String|Split (Variables|/Game/Blueprints/BP_GlobalSave.BP_GlobalSave_C|GetLast%20Level%20Played _asbp_global_save) "_")) "infinitymode")
      (Public|MoveNoAnim 1 (+ (CallFunction|GetAmountOfSeasons) 1))
      (else
        (bind (_array_element _array_index) (Utilities|Array|ForEachLoopwithBreak (CallFunction|GetSeasonNames))
          (:LoopBody
            (if (Utilities|Enum|Equal(Enum) _array_element (.LeftS (Utilities|String|Split (Variables|/Game/Blueprints/BP_GlobalSave.BP_GlobalSave_C|GetLast%20Level%20Played _asbp_global_save) "_")))
              (Public|MoveNoAnim 1 (+ _array_index 1)))))))))

(fn Move
  (params (Koef :type Float%20%28single-precision%29) (Sprite :type Paper%20Sprite%20Component%20Object%20Reference))
  (Transformation|SetRelativeLocation Sprite (Math|Vector|MakeVector 0.0 (.Y (Math|Vector|BreakVector (Variables|/Script/Engine.SceneComponent|GetRelativeLocation Sprite))) (* (* (Variables|Default|GetVer%20Position) -8e+02) Koef)) false false))

(fn MoveNoAnim
  (params (Vertical :type Integer) (Horisontal :type Integer))
  (Utilities|FlowControl|Sequence
    (:then_0
      (switch int Vertical
        (:0
          (Variables|Default|SetVer%20Position 1.0))
        (:1
          (Variables|Default|SetVer%20Position 0.5))
        (:2
          (Variables|Default|SetVer%20Position 0.0)))
      (Variables|Default|SetHor%20Position Horisontal))
    (:then_1
      (Transformation|SetActorLocation (Math|Vector|MakeVector (- 2.6e+03 (* (/ (Math|Conversions|ToFloat(Integer) Horisontal) (Math|Conversions|ToFloat(Integer) (+ (CallFunction|GetAmountOfSeasons) 2))) 5.2e+03)) -3e+03 0.0) false false))))

(fn OnRepPos
  (for (_array_element _array_index) (Variables|Default|GetSprites)
    (Private|Move (* _array_index 0.3) _array_element)))

(fn Refresh
  (params (Update%20Loc :type Boolean))
  (bind _amount (CallFunction|GetAmountOfSeasons))
  (bind _sprites (Variables|Default|GetSprites))
  (bind _returnvalue (+ _amount 2))
  (bind _result (CallFunction|GetMenuSeason))
  (bind _output_get (Variables|Default|SetSeason _result))
  (for _array_element _sprites
    (Components|DestroyComponent _array_element))
  (Utilities|Array|Clear _sprites)
  (for (_array_element_2 _array_index) (CallFunction|GetParallaxSpritesbySeason _output_get)
    (bind _returnvalue_2 (AddComponent|AddPaperSpriteComponent false (Math|Transform|MakeTransform (Math|Vector|MakeVector 0.0 (+ (* _array_index 6e+02) -2e+03) 0.0))))
    (Utilities|Array|Add (Variables|Default|GetSprites) _returnvalue_2)
    (Rendering|Components|Sprite|SetSprite _returnvalue_2 _array_element_2))
  (if Update%20Loc
    (Variables|Default|SetVer%20Position (Variables|Default|GetVer%20Position))
    (Transformation|SetActorLocation (Math|Vector|MakeVector (- (* (/ (Math|Conversions|ToFloat(Integer) (- _returnvalue (Variables|Default|GetHor%20Position))) (Math|Conversions|ToFloat(Integer) _returnvalue)) 5.2e+03) 2.6e+03) -3e+03 0.0) false false)))

(fn SetVertical
  (params (Ver :type Integer))
  (switch int Ver
    (:0
      (CallFunction|MoveVer 1.0))
    (:1
      (CallFunction|MoveVer 0.5))
    (:2
      (CallFunction|MoveVer 0.0))))

(fn SetHorizontal
  (params (Horizontal :type Integer))
  (bind _output_get (Variables|Default|SetHor%20Position Horizontal))
  (CallFunction|MoveHor _output_get))