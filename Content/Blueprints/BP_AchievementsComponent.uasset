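; Achievements component that tracks player gameplay statistics and unlocks achievements.
; On BeginPlay it finds the main character and binds to events for deaths, spawns, respawns, teleports, pickups, level completion, destroyed platforms and Infinity Mode.
; Each handler increments its stat via AdjustStat, with Infinity Mode movement scaled down and rounded.
; Only deaths and spawns check the updated total against tiered thresholds to call CompleteAchievement.
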(event Custom|Event%20Dead
  ;[1 1 1] Death
  (bind _returnvalue (CallFunction|AdjustStat "NewEnumerator0" 1))
  (Utilities|FlowControl|Sequence
    (:then_0
      (if (>= _returnvalue 5)
        (CallFunction|CompleteAchievement "NewEnumerator0")))
    (:then_1
      (if (>= _returnvalue 100)
        (CallFunction|CompleteAchievement "NewEnumerator2")))
    (:then_2
      (if (>= _returnvalue 1000)
        (CallFunction|CompleteAchievement "NewEnumerator4")))))

(event Custom|Event%20Spawn
  ;[1 1 1] Spawn
  (bind _returnvalue (CallFunction|AdjustStat "NewEnumerator1" 1))
  (Utilities|FlowControl|Sequence
    (:then_0
      (if (>= _returnvalue 5)
        (CallFunction|CompleteAchievement "NewEnumerator1")))
    (:then_1
      (if (>= _returnvalue 12)
        (CallFunction|CompleteAchievement "NewEnumerator3")))
    (:then_2
      (if (>= _returnvalue 1000)
        (CallFunction|CompleteAchievement "NewEnumerator5")))))

(event Custom|Event%20Platform%20Destroyed
  ;[1 1 1] Platforms Destroyed
  (CallFunction|AdjustStat "NewEnumerator10" 1))

(event Custom|Event%20Respawn
  ;[1 1 1] Respawn
  (CallFunction|AdjustStat "NewEnumerator2" 1))

(event Custom|Event%20Teleport
  ;[1 1 1] Teleported
  (CallFunction|AdjustStat "NewEnumerator3" 1))

(event Custom|Event%20Shield%20Picked
  ;[1 1 1] Shields Picked
  (CallFunction|AdjustStat "NewEnumerator4" 1))

(event Custom|Event%20Boost%20Picked
  ;[1 1 1] Boosts Picked
  (CallFunction|AdjustStat "NewEnumerator5" 1))

(event Custom|Event%20Star%20Picked
  ;[1 1 1] Star Collected
  (CallFunction|AdjustStat "NewEnumerator6" 1))

(event Custom|Event%20Level%20Complete
  ;[1 1 1] Levels Completed
  (CallFunction|AdjustStat "NewEnumerator7" 1))

(event Custom|Event%20Move%20in%20Infinity%20Mode
  (params (Movement :type Float%20%28single-precision%29))
  ;[1 1 1] Points in Infinity Mode
  (CallFunction|AdjustStat "NewEnumerator8" (Math|Float|Round (/ Movement 1e+01))))

(event Custom|Event%20Spawn%20Infinity%20Mode
  ;[1 1 1] Spawns in Infinity Mode
  (CallFunction|AdjustStat "NewEnumerator9" 1))

(event EventBeginPlay
  (bind _outactors (Actor|GetAllActorsOfClass "/Game/Blueprints/Characters/BP_Character_Main.BP_Character_Main_C"))
  (bind _output_get (Variables|Default|SetCharacter (Utilities|Array|Get(acopy) _outactors)))
  (EventDispatchers|AssignEventDead _output_get (delegate Custom|Event%20Dead))
  (EventDispatchers|BindEventtoEventSpawn _output_get (delegate Custom|Event%20Spawn))
  (EventDispatchers|BindEventtoEventRespawn (delegate Custom|Event%20Respawn))
  (EventDispatchers|BindEventtoEventTeleport (delegate Custom|Event%20Teleport))
  (EventDispatchers|BindEventtoEventShieldPickup (delegate Custom|Event%20Shield%20Picked))
  (EventDispatchers|BindEventtoEventBoostPickup (delegate Custom|Event%20Boost%20Picked))
  (EventDispatchers|BindEventtoEventStarsPickedUp (delegate Custom|Event%20Star%20Picked))
  (EventDispatchers|BindEventtoEventLevelComplete (delegate Custom|Event%20Level%20Complete))
  (EventDispatchers|BindEventtoEventMoveinInfinityMode (delegate Custom|Event%20Move%20in%20Infinity%20Mode))
  (EventDispatchers|BindEventtoEventSpawnInfinityMode (delegate Custom|Event%20Spawn%20Infinity%20Mode))
  (EventDispatchers|BindEventtoEventDestroyedPlatform (delegate Custom|Event%20Platform%20Destroyed)))