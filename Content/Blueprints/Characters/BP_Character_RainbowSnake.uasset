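; BP_Character_RainbowSnake is a snake character variant whose head sprite and trail continuously cycle through rainbow colors.
; After the parent Tick, it advances the PaperSprite's hue by DeltaSeconds at a fixed rate, wrapping at 365 rather than 360, with full saturation and value.
; Each Trail element's CubeSprite derives its color from the updated head hue plus the same increment, so the trail shares one color slightly ahead of the head.
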(event EventBeginPlay
  (|CallParentFunction) ; This node is disabled and will not be called.\nDrag off pins to build functionality.
)

(event Collision|EventActorBeginOverlap
  (params (OtherActor :type Actor%20Object%20Reference)))

(event EventTick
  (params (DeltaSeconds :type Float%20%28single-precision%29))
  (bind _returnvalue (* DeltaSeconds 1e+02))
  (bind _papersprite (Variables|Default|GetPaperSprite))
  (bind _spritecolor (Variables|/Script/Paper2D.PaperSpriteComponent|GetSpriteColor _papersprite))
  (bind _h (Math|Color|RGBtoHSV(LinearColor) _spritecolor))
  (bind _returnvalue_2 (+ _h _returnvalue))
  (bind _returnvalue_3 (Math|Float|%(Float) _returnvalue_2 365.0))
  (bind _returnvalue_4 (Class|KismetMathLibrary|HSVtoRGB _returnvalue_3 1.0 1.0 1.0))
  (|CallParentFunction DeltaSeconds)
  (Sprite|SetSpriteColor _papersprite _returnvalue_4)
  (for _array_element (Variables|Default|GetTrail)
    (Sprite|SetSpriteColor (Variables|/Game/Blueprints/BP_Trail.BP_Trail_C|GetCubeSprite _array_element) _returnvalue_4)))

(fn ConstructionScript
  (|CallParentFunction))