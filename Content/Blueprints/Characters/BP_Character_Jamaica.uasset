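; Jamaica character variant that recolors the trail of cube sprites it uses from its parent class.
; On BeginPlay, after the parent logic, it loops over the Trail array and tints each element's CubeSprite yellow, red, near-black or green.
; Integer division and modulo on the offset index make the colors repeat in two-element bands, with a single yellow element at the start.
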(event EventBeginPlay
  (|CallParentFunction)
  (for (_array_element _array_index) (Variables|Default|GetTrail)
    (switch int (Math|Integer|%(Integer) (/ (- _array_index -1) 2) 4)
      (:0
        (Sprite|SetSpriteColor (Variables|/Game/Blueprints/BP_Trail.BP_Trail_C|GetCubeSprite _array_element) "(R=1.000000,G=1.000000,B=0.000000,A=1.000000)"))
      (:1
        (Sprite|SetSpriteColor (Variables|/Game/Blueprints/BP_Trail.BP_Trail_C|GetCubeSprite _array_element) "(R=1.000000,G=0.000000,B=0.000000,A=1.000000)"))
      (:2
        (Sprite|SetSpriteColor (Variables|/Game/Blueprints/BP_Trail.BP_Trail_C|GetCubeSprite _array_element) "(R=0.104167,G=0.104167,B=0.104167,A=1.000000)"))
      (:3
        (Sprite|SetSpriteColor (Variables|/Game/Blueprints/BP_Trail.BP_Trail_C|GetCubeSprite _array_element) "(R=0.000000,G=1.000000,B=0.000000,A=1.000000)")))))

(event Collision|EventActorBeginOverlap
  (params (OtherActor :type Actor%20Object%20Reference)))

(event EventTick
  (params (DeltaSeconds :type Float%20%28single-precision%29))
  (|CallParentFunction DeltaSeconds) ; This node is disabled and will not be called.\nDrag off pins to build functionality.
)

(fn ConstructionScript
  (|CallParentFunction))