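; Player character for a side-view game that flies constantly along a steerable Look vector, trailed by a chain of follower actors.
; Tick drives sweep movement, distance, timer and clamped camera; a missing finish line selects infinity mode.
; Pickups orbit the player, with shields destroying platforms or doors on impact; otherwise hits and leaving bounds trigger the lose screen.
; Macros handle a save-gated intro camera pan and portal teleports with camera catch-up.
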(event Custom|Event%20Hit
  (params (NewVar_0 :type Actor%20Object%20Reference))
  (bind _returnvalue (Game|GetPlayerController 0))
  ;[1 1 1] Hitting Something
  (Variables|Default|SetNewVar_0 NewVar_0)
  (if (Math|Boolean|ORBoolean (== "/Game/Blueprints/LevelStuff/BP_Platform.BP_Platform_C" (Utilities|GetClass (Variables|Default|GetNewVar_0))) (== "/Game/Blueprints/LevelStuff/BP_LockedDoor.BP_LockedDoor_C" (Utilities|GetClass (Variables|Default|GetNewVar_0))) (== "/Game/Blueprints/LevelStuff/BP_MovingPlatform.BP_MovingPlatform_C" (Utilities|GetClass (Variables|Default|GetNewVar_0))))
    (bind _filteredarray (Utilities|Array|FilterArray (Variables|Default|GetInteractables) "/Game/Blueprints/Interactables/BP_Shield.BP_Shield_C"))
    (if (!= (Utilities|Array|Length _filteredarray) 0)
      ;;[1 1 1] Shield Trigger
      (Actor|DestroyActor (Variables|Default|GetNewVar_0))
      (Default|CallEventDestroyedPlatform)
      (CallFunction|RemoveInteractable (.AsBP%20Shield (Utilities|Casting|CastToBP_Shield (Utilities|Array|Get(acopy) _filteredarray))))
      (bind _returnvalue_2 (Audio|SpawnSound2D "/Engine/VREditor/Sounds/UI/Floating_UI_Close.Floating_UI_Close" 1.0 1.0 0.0 0))
      (Audio|Components|Audio|Play _returnvalue_2 0.0)
      (else
        ;;[1 1 1] Death
        (Utilities|FlowControl|DoOnce false :!label _label
          (:Completed
            (Default|CallEventDead)
            (Utilities|FlowControl|Sequence
              (:then_0
                (Effects|SpawnEmitterAttached "/Game/Effects/Effects/FX_Monsters/FX_Monster_Gruntling/Notifies/P_Death_backpack_expl_02.P_Death_backpack_expl_02" (Variables|Collision|GetCapsuleComponent) "None")
                (bind _returnvalue_3 (Audio|CreateSound2D "/Engine/VREditor/Sounds/UI/Dockable_Window_Close.Dockable_Window_Close" 1.0 1.0 0.0 0))
                (Audio|Components|Audio|Play _returnvalue_3 0.0)
                (Utilities|FlowControl|Delay 0.4)
                (Game|SetGamePaused true)
                (if (Variables|Default|GetInfinity%20Mode)
                  (bind _returnvalue_4 (UserInterface|CreateWidget "/Game/Blueprints/Widgets/InfinityMode/W_InfinityLooseScreen.W_InfinityLooseScreen_C" (Game|GetPlayerController 0) (Utilities|Text|ToText(Float) (/ (Variables|Default|GetCurrentDistance) 1e+01) "HalfToEven" false true 1 324 0 0)))
                  (UserInterface|Viewport|AddtoPlayerScreen _returnvalue_4)
                  (else
                    (bind _returnvalue_5 (UserInterface|CreateWidget "/Game/Blueprints/Widgets/StandartMode/W_LooseScreen.W_LooseScreen_C" _returnvalue))
                    (UserInterface|Viewport|AddtoPlayerScreen _returnvalue_5)))
                (Variables|/Script/Engine.PlayerController|SetbShowMouseCursor _returnvalue true)
                (bind _foundwidgets (Widget|GetAllWidgetsOfClass "/Game/Blueprints/Widgets/StandartMode/W_Interface.W_Interface_C" true))
                (for _array_element _foundwidgets
                  (Widget|RemovefromParent _array_element))
                (bind _foundwidgets_2 (Widget|GetAllWidgetsOfClass "/Game/Blueprints/Widgets/InfinityMode/W_InfinityInterface.W_InfinityInterface_C" true))
                (for _array_element_2 _foundwidgets_2
                  (Widget|RemovefromParent _array_element_2)))
              (:then_1
                (Variables|Default|SetSpeed 0.0)))))))
    (else
      (goto _label))))

(event Custom|Respawn
  (bind _returnvalue (Game|GetPlayerController 0))
  ;[1 1 1] Respawn
  (Default|CallEventRespawn)
  (Variables|Default|SetSpeed 6e+02)
  ;[1 1 1] Hitting Something
  ;;[1 1 1] Death
  (Utilities|FlowControl|DoOnce false) ; enters at Reset
)

(event Custom|Rotate
  (params (A :type Float%20%28single-precision%29))
  (bind _returnvalue (Utilities|Time|GetWorldDeltaSeconds))
  (bind _rotspeed (Variables|Default|GetRotSpeed))
  (bind _returnvalue_2 (* A _rotspeed _returnvalue 5e+01))
  (bind _returnvalue_3 (* _returnvalue_2 -1.0))
  ;[1 1 1] Movement
  (Utilities|FlowControl|Gate true
    (:Exit
      (Variables|Default|SetLook (Math|Vector|RotateVectorAroundAxis (Variables|Default|GetLook) _returnvalue_2 "0,1.000000, 0"))
      (if (Variables|SkinSettings|GetRotateHead)
        (Transformation|AddWorldRotation (Variables|Default|GetPaperSprite) (Math|Rotator|MakeRotator 0.0 _returnvalue_3 0.0) false false))
      (if (Variables|SkinSettings|GetRotateTrail)
        (for (_array_element _array_index) (Variables|Default|GetTrail)
          (switch int (Math|Integer|%(Integer) _array_index 2)
            (:0
              (Class|Actor|AddActorWorldRotation _array_element (Math|Rotator|MakeRotator 0.0 _returnvalue_3 0.0)))
            (:1
              (Class|Actor|AddActorWorldRotation _array_element (Math|Rotator|MakeRotator 0.0 _returnvalue_2 0.0)))))))))

(event Custom|PortalTeleport
  (params (From :type Vector) (To :type Vector))
  ;[1 1 1] Teleportation
  (Default|CallEventTeleport)
  (Utilities|Teleport From To))

(event EventBeginPlay
  (bind _returnvalue (Game|GetPlayerController 0))
  (bind _self self)
  (bind _self_2 self)
  (bind _self_3 self)
  (bind _self_4 self)
  (bind _trail (Variables|Default|GetTrail))
  (bind _sideviewcameracomponent (Variables|Camera|GetSideViewCameraComponent))
  (bind _trailsprite (Variables|SkinSettings|GetTrailSprite))
  (bind _trail_color (Variables|SkinSettings|GetTrail%20Color))
  (bind _trailclass (Variables|SkinSettings|GetTrailClass))
  (bind _papersprite (Variables|Default|GetPaperSprite))
  (bind _sideviewcameracomponent_2 (Variables|Camera|GetSideViewCameraComponent))
  (bind _returnvalue_2 (Transformation|GetActorLocation _self_4))
  (bind _returnvalue_3 (Transformation|GetActorTransform _self_2))
  (bind _returnvalue_4 (Transformation|GetActorLocation _self))
  (bind (_x _y _z) (Math|Vector|BreakVector _returnvalue_2))
  (bind _z_2 (Math|Vector|BreakVector _returnvalue_4))
  (bind (_location _rotation) (Math|Transform|BreakTransform _returnvalue_3))
  (bind (_x_2 _y_2 _z_3) (Math|Vector|BreakVector _location))
  (Default|CallEventSpawn)
  (if (Variables|Default|GetInfinity%20Mode)
    (Default|CallEventSpawnInfinityMode))
  (Utilities|FlowControl|Sequence
    (:then_0
      ;[1 1 1] Updating Topscreen bar
      (bind _outactors (Actor|GetAllActorsOfClass "/Game/Blueprints/LevelStuff/BP_FinishLine.BP_FinishLine_C"))
      (Utilities|IsValid (Utilities|Array|Get(acopy) _outactors)
        (:Is%20Valid
          (Variables|Default|SetCurrentDistance (- (.Z (Math|Vector|BreakVector (Transformation|GetActorLocation (Utilities|Array|Get(acopy) _outactors)))) _z_2)))
        (:Is%20Not%20Valid
          (if (> (- _z_2 (Variables|Default|GetDistanceToFinish)) (Variables|Default|GetCurrentDistance))
            (Variables|Default|SetCurrentDistance (- _z_2 (Variables|Default|GetDistanceToFinish))))))
      ;[1 1 1] Timer Update
      (Variables|Default|SetTime (Math|Timespan|MakeTimespan (.Days (Math|Timespan|BreakTimespan (Variables|Default|GetTime))) (.Hours (Math|Timespan|BreakTimespan (Variables|Default|GetTime))) (.Minutes (Math|Timespan|BreakTimespan (Variables|Default|GetTime))) (.Seconds (Math|Timespan|BreakTimespan (Variables|Default|GetTime))) (+ (Math|Float|Truncate (* (stale EventTick DeltaSeconds) 1e+03)) (.Milliseconds (Math|Timespan|BreakTimespan (Variables|Default|GetTime))))))
      ;[1 1 1] Moving and screenborder collision
      (if (Variables|Default|GetInfinity%20Mode)
        (Default|CallEventMoveinInfinityMode (* (stale EventTick DeltaSeconds) (Variables|Default|GetSpeed))))
      (bind _sweephitresult (Transformation|SetActorLocation self (+ (* (Variables|Default|GetLook) (* (stale EventTick DeltaSeconds) (Variables|Default|GetSpeed))) _returnvalue_2) true false))
      (if (Math|Boolean|ORBoolean (<= _x -1e+03) (>= _x 1e+03) (<= _z -1.3e+03))
        ;[1 1 1] Hitting Something
        ;;[1 1 1] Death
        (Utilities|FlowControl|DoOnce false :!label _label
          (:Completed
            (Default|CallEventDead)
            (Utilities|FlowControl|Sequence
              (:then_0
                (Effects|SpawnEmitterAttached "/Game/Effects/Effects/FX_Monsters/FX_Monster_Gruntling/Notifies/P_Death_backpack_expl_02.P_Death_backpack_expl_02" (Variables|Collision|GetCapsuleComponent) "None")
                (bind _returnvalue_5 (Audio|CreateSound2D "/Engine/VREditor/Sounds/UI/Dockable_Window_Close.Dockable_Window_Close" 1.0 1.0 0.0 0))
                (Audio|Components|Audio|Play _returnvalue_5 0.0)
                (Utilities|FlowControl|Delay 0.4)
                (Game|SetGamePaused true)
                (if (Variables|Default|GetInfinity%20Mode)
                  (bind _returnvalue_6 (UserInterface|CreateWidget "/Game/Blueprints/Widgets/InfinityMode/W_InfinityLooseScreen.W_InfinityLooseScreen_C" (Game|GetPlayerController 0) (Utilities|Text|ToText(Float) (/ (Variables|Default|GetCurrentDistance) 1e+01) "HalfToEven" false true 1 324 0 0)))
                  (UserInterface|Viewport|AddtoPlayerScreen _returnvalue_6)
                  (else
                    (bind _returnvalue_7 (UserInterface|CreateWidget "/Game/Blueprints/Widgets/StandartMode/W_LooseScreen.W_LooseScreen_C" _returnvalue))
                    (UserInterface|Viewport|AddtoPlayerScreen _returnvalue_7)))
                (Variables|/Script/Engine.PlayerController|SetbShowMouseCursor _returnvalue true)
                (bind _foundwidgets (Widget|GetAllWidgetsOfClass "/Game/Blueprints/Widgets/StandartMode/W_Interface.W_Interface_C" true))
                (for _array_element _foundwidgets
                  (Widget|RemovefromParent _array_element))
                (bind _foundwidgets_2 (Widget|GetAllWidgetsOfClass "/Game/Blueprints/Widgets/InfinityMode/W_InfinityInterface.W_InfinityInterface_C" true))
                (for _array_element_2 _foundwidgets_2
                  (Widget|RemovefromParent _array_element_2)))
              (:then_1
                (Variables|Default|SetSpeed 0.0)))))
        (else
          ;[1 1 1] Interactables
          (for _array_element_3 (Variables|Default|GetInteractables)
            (Utilities|IsValid _array_element_3
              (:Is%20Valid
                (Transformation|SetActorLocation _array_element_3 (+ (Transformation|GetActorLocation _array_element_3) (* (Variables|Default|GetLook) (* (stale EventTick DeltaSeconds) (Variables|Default|GetSpeed)))) false true)
                (Transformation|SetActorLocation _array_element_3 (+ (Transformation|GetActorLocation _array_element_3) (Math|Vector|RotateVectorAroundAxis (- (Transformation|GetActorLocation _array_element_3) (Transformation|GetActorLocation self)) (/ 6.0 (Math|Conversions|ToFloat(Integer) (+ (Utilities|Array|Length (Variables|Default|GetInteractables)) 1))) "0,1.000000, 0") (- "0, 0, 0" (- (Transformation|GetActorLocation _array_element_3) (Transformation|GetActorLocation self)))) false true))))
          (Variables|Default|SetNewVar_0 (.HitActor (Collision|BreakHitResult _sweephitresult)))
          (if (.bBlockingHit (Collision|BreakHitResult _sweephitresult))
            (if (Math|Boolean|ORBoolean (== "/Game/Blueprints/LevelStuff/BP_Platform.BP_Platform_C" (Utilities|GetClass (Variables|Default|GetNewVar_0))) (== "/Game/Blueprints/LevelStuff/BP_LockedDoor.BP_LockedDoor_C" (Utilities|GetClass (Variables|Default|GetNewVar_0))) (== "/Game/Blueprints/LevelStuff/BP_MovingPlatform.BP_MovingPlatform_C" (Utilities|GetClass (Variables|Default|GetNewVar_0))))
              (bind _filteredarray (Utilities|Array|FilterArray (Variables|Default|GetInteractables) "/Game/Blueprints/Interactables/BP_Shield.BP_Shield_C"))
              (if (!= (Utilities|Array|Length _filteredarray) 0)
                ;;[1 1 1] Shield Trigger
                (Actor|DestroyActor (Variables|Default|GetNewVar_0))
                (Default|CallEventDestroyedPlatform)
                (CallFunction|RemoveInteractable (.AsBP%20Shield (Utilities|Casting|CastToBP_Shield (Utilities|Array|Get(acopy) _filteredarray))))
                (bind _returnvalue_8 (Audio|SpawnSound2D "/Engine/VREditor/Sounds/UI/Floating_UI_Close.Floating_UI_Close" 1.0 1.0 0.0 0))
                (Audio|Components|Audio|Play _returnvalue_8 0.0)
                (else
                  (goto _label)))
              (else
                (goto _label)))
            (else
              ;[1 1 1] Camera
              (if (Variables|Default|GetInfinity%20Mode)
                (if (Variables|Default|GetTeleporting)
                  (Transformation|SetWorldLocation _sideviewcameracomponent (Math|Vector|MakeVector 0.0 5e+02 (Math|Float|Clamp(Float) (Variables|Default|GetNewVar_4) 5e+02 1e+07)) false true)
                  (else
                    (Transformation|SetWorldLocation _sideviewcameracomponent (Math|Vector|MakeVector 0.0 5e+02 (Math|Float|Clamp(Float) (.Z (Math|Vector|BreakVector (Transformation|GetActorLocation self))) 5e+02 1e+07)) false true)))
                (elif (Variables|Default|GetTeleporting)
                  (Transformation|SetWorldLocation _sideviewcameracomponent_2 (Math|Vector|MakeVector 0.0 5e+02 (Math|Float|Clamp(Float) (Variables|Default|GetNewVar_4) 5e+02 2.2e+03)) false true)
                  (else
                    (Transformation|SetWorldLocation _sideviewcameracomponent_2 (Math|Vector|MakeVector 0.0 5e+02 (Math|Float|Clamp(Float) (.Z (Math|Vector|BreakVector (Transformation|GetActorLocation self))) 5e+02 2.2e+03)) false true)))))))))
    (:then_1
      ;[1 1 1] Skin Initialisation
      (Rendering|Components|Sprite|SetSprite _papersprite (Variables|SkinSettings|GetMain%20Sprite))
      (Sprite|SetSpriteColor _papersprite (Variables|SkinSettings|GetMain%20Sprite%20Color))
      ;[1 1 1] Train inicialisation
      (for _index (range 1 (Variables|SkinSettings|GetTrailLength))
        (if (== _index 1)
          (bind _returnvalue_9 (Game|SpawnActorfromClass _trailclass (Math|Transform|MakeTransform (Math|Vector|MakeVector _x_2 (+ (* -1.0 (Math|Conversions|ToFloat(Integer) (+ _index 1))) -7e+01) _z_3) _rotation (Math|Vector|MakeVector (* (/ 1.0 (Math|Float|Sqrt (Math|Conversions|ToFloat(Integer) (+ _index 1)))) (Variables|SkinSettings|GetTrailScale)) (* (/ 1.0 (Math|Float|Sqrt (Math|Conversions|ToFloat(Integer) (+ _index 1)))) (Variables|SkinSettings|GetTrailScale)) (* (/ 1.0 (Math|Float|Sqrt (Math|Conversions|ToFloat(Integer) (+ _index 1)))) (Variables|SkinSettings|GetTrailScale)))) "Undefined" 0 _self_3 (* (/ 1.0 (Math|Float|Sqrt (Math|Conversions|ToFloat(Integer) (+ _index 1)))) 1.2e+02) _trailsprite _trail_color _self_3))
          (Utilities|Array|Add _trail _returnvalue_9)
          (else
            (bind _returnvalue_10 (Game|SpawnActorfromClass _trailclass (Math|Transform|MakeTransform (Math|Vector|MakeVector _x_2 (+ (* -1.0 (Math|Conversions|ToFloat(Integer) (+ _index 1))) -7e+01) _z_3) _rotation (Math|Vector|MakeVector (* (/ 1.0 (Math|Float|Sqrt (Math|Conversions|ToFloat(Integer) (+ _index 1)))) (Variables|SkinSettings|GetTrailScale)) (* (/ 1.0 (Math|Float|Sqrt (Math|Conversions|ToFloat(Integer) (+ _index 1)))) (Variables|SkinSettings|GetTrailScale)) (* (/ 1.0 (Math|Float|Sqrt (Math|Conversions|ToFloat(Integer) (+ _index 1)))) (Variables|SkinSettings|GetTrailScale)))) "Undefined" 0 (Utilities|Array|Get(acopy) _trail (- _index 2)) (* (/ 1.0 (Math|Float|Sqrt (Math|Conversions|ToFloat(Integer) (+ _index 1)))) 1.2e+02) _trailsprite _trail_color _self_3))
            (Utilities|Array|Add _trail _returnvalue_10))))
      (Variables|Default|SetRotSpeed 4.0)
      ;[1 1 1] Interface inicialisation
      (bind _outactors_2 (Actor|GetAllActorsOfClass "/Game/Blueprints/LevelStuff/BP_FinishLine.BP_FinishLine_C"))
      (Utilities|IsValid (Utilities|Array|Get(acopy) _outactors_2)
        (:Is%20Valid
          (Variables|Default|SetDistanceToFinish (- (- (.Z (Math|Vector|BreakVector (Transformation|GetActorLocation (Utilities|Array|Get(acopy) _outactors_2)))) (.Z (Math|Vector|BreakVector (Transformation|GetActorLocation self)))) 1e+02))
          (bind _returnvalue_11 (UserInterface|CreateWidget "/Game/Blueprints/Widgets/StandartMode/W_Interface.W_Interface_C" (Game|GetPlayerController 0)))
          (UserInterface|Viewport|AddtoViewport _returnvalue_11 0)
          (Variables|Default|SetInfinity%20Mode false))
        (:Is%20Not%20Valid
          (Variables|Default|SetDistanceToFinish (.Z (Math|Vector|BreakVector (Transformation|GetActorLocation self))))
          (bind _returnvalue_12 (UserInterface|CreateWidget "/Game/Blueprints/Widgets/InfinityMode/W_InfinityInterface.W_InfinityInterface_C" (Game|GetPlayerController 0)))
          (UserInterface|Viewport|AddtoViewport _returnvalue_12 0)
          (Variables|Default|SetInfinity%20Mode true))))
    (:then_2
      ;[1 1 1] Camera Anim
      (|BeginCamera
        (:then_12
          (Utilities|FlowControl|Sequence
            (:then_0
              (Utilities|FlowControl|Gate true) ; enters at Open
            )
            (:then_1
              ;[1 1 1] Movement
              (Utilities|FlowControl|Gate true) ; enters at Open
            )
            (:then_2
              (Utilities|FlowControl|Gate true) ; enters at Open
            )))))))

(event EventTick
  (params (DeltaSeconds :type Float%20%28single-precision%29))
  (bind _returnvalue (Game|GetPlayerController 0))
  (bind _self self)
  (bind _self_2 self)
  (bind _distancetofinish (Variables|Default|GetDistanceToFinish))
  (bind _sideviewcameracomponent (Variables|Camera|GetSideViewCameraComponent))
  (bind _sideviewcameracomponent_2 (Variables|Camera|GetSideViewCameraComponent))
  (bind _returnvalue_2 (Transformation|GetActorLocation _self_2))
  (bind _returnvalue_3 (Transformation|GetActorLocation _self))
  (bind (_x _y _z) (Math|Vector|BreakVector _returnvalue_2))
  (bind _z_2 (Math|Vector|BreakVector _returnvalue_3))
  (bind _returnvalue_4 (- _z_2 _distancetofinish))
  (Utilities|FlowControl|Gate true
    (:Exit
      ;[1 1 1] Updating Topscreen bar
      (bind _outactors (Actor|GetAllActorsOfClass "/Game/Blueprints/LevelStuff/BP_FinishLine.BP_FinishLine_C"))
      (Utilities|IsValid (Utilities|Array|Get(acopy) _outactors)
        (:Is%20Valid
          (Variables|Default|SetCurrentDistance (- (.Z (Math|Vector|BreakVector (Transformation|GetActorLocation (Utilities|Array|Get(acopy) _outactors)))) _z_2)))
        (:Is%20Not%20Valid
          (if (> _returnvalue_4 (Variables|Default|GetCurrentDistance))
            (Variables|Default|SetCurrentDistance _returnvalue_4))))
      ;[1 1 1] Timer Update
      (Variables|Default|SetTime (Math|Timespan|MakeTimespan (.Days (Math|Timespan|BreakTimespan (Variables|Default|GetTime))) (.Hours (Math|Timespan|BreakTimespan (Variables|Default|GetTime))) (.Minutes (Math|Timespan|BreakTimespan (Variables|Default|GetTime))) (.Seconds (Math|Timespan|BreakTimespan (Variables|Default|GetTime))) (+ (Math|Float|Truncate (* DeltaSeconds 1e+03)) (.Milliseconds (Math|Timespan|BreakTimespan (Variables|Default|GetTime))))))
      ;[1 1 1] Moving and screenborder collision
      (if (Variables|Default|GetInfinity%20Mode)
        (Default|CallEventMoveinInfinityMode (* DeltaSeconds (Variables|Default|GetSpeed))))
      (bind _sweephitresult (Transformation|SetActorLocation self (+ (* (Variables|Default|GetLook) (* DeltaSeconds (Variables|Default|GetSpeed))) _returnvalue_2) true false))
      (if (Math|Boolean|ORBoolean (<= _x -1e+03) (>= _x 1e+03) (<= _z -1.3e+03))
        ;[1 1 1] Hitting Something
        ;;[1 1 1] Death
        (Utilities|FlowControl|DoOnce false :!label _label
          (:Completed
            (Default|CallEventDead)
            (Utilities|FlowControl|Sequence
              (:then_0
                (Effects|SpawnEmitterAttached "/Game/Effects/Effects/FX_Monsters/FX_Monster_Gruntling/Notifies/P_Death_backpack_expl_02.P_Death_backpack_expl_02" (Variables|Collision|GetCapsuleComponent) "None")
                (bind _returnvalue_5 (Audio|CreateSound2D "/Engine/VREditor/Sounds/UI/Dockable_Window_Close.Dockable_Window_Close" 1.0 1.0 0.0 0))
                (Audio|Components|Audio|Play _returnvalue_5 0.0)
                (Utilities|FlowControl|Delay 0.4)
                (Game|SetGamePaused true)
                (if (Variables|Default|GetInfinity%20Mode)
                  (bind _returnvalue_6 (UserInterface|CreateWidget "/Game/Blueprints/Widgets/InfinityMode/W_InfinityLooseScreen.W_InfinityLooseScreen_C" (Game|GetPlayerController 0) (Utilities|Text|ToText(Float) (/ (Variables|Default|GetCurrentDistance) 1e+01) "HalfToEven" false true 1 324 0 0)))
                  (UserInterface|Viewport|AddtoPlayerScreen _returnvalue_6)
                  (else
                    (bind _returnvalue_7 (UserInterface|CreateWidget "/Game/Blueprints/Widgets/StandartMode/W_LooseScreen.W_LooseScreen_C" _returnvalue))
                    (UserInterface|Viewport|AddtoPlayerScreen _returnvalue_7)))
                (Variables|/Script/Engine.PlayerController|SetbShowMouseCursor _returnvalue true)
                (bind _foundwidgets (Widget|GetAllWidgetsOfClass "/Game/Blueprints/Widgets/StandartMode/W_Interface.W_Interface_C" true))
                (for _array_element _foundwidgets
                  (Widget|RemovefromParent _array_element))
                (bind _foundwidgets_2 (Widget|GetAllWidgetsOfClass "/Game/Blueprints/Widgets/InfinityMode/W_InfinityInterface.W_InfinityInterface_C" true))
                (for _array_element_2 _foundwidgets_2
                  (Widget|RemovefromParent _array_element_2)))
              (:then_1
                (Variables|Default|SetSpeed 0.0)))))
        (else
          ;[1 1 1] Interactables
          (for _array_element_3 (Variables|Default|GetInteractables)
            (Utilities|IsValid _array_element_3
              (:Is%20Valid
                (Transformation|SetActorLocation _array_element_3 (+ (Transformation|GetActorLocation _array_element_3) (* (Variables|Default|GetLook) (* DeltaSeconds (Variables|Default|GetSpeed)))) false true)
                (Transformation|SetActorLocation _array_element_3 (+ (Transformation|GetActorLocation _array_element_3) (Math|Vector|RotateVectorAroundAxis (- (Transformation|GetActorLocation _array_element_3) (Transformation|GetActorLocation self)) (/ 6.0 (Math|Conversions|ToFloat(Integer) (+ (Utilities|Array|Length (Variables|Default|GetInteractables)) 1))) "0,1.000000, 0") (- "0, 0, 0" (- (Transformation|GetActorLocation _array_element_3) (Transformation|GetActorLocation self)))) false true))))
          (Variables|Default|SetNewVar_0 (.HitActor (Collision|BreakHitResult _sweephitresult)))
          (if (.bBlockingHit (Collision|BreakHitResult _sweephitresult))
            (if (Math|Boolean|ORBoolean (== "/Game/Blueprints/LevelStuff/BP_Platform.BP_Platform_C" (Utilities|GetClass (Variables|Default|GetNewVar_0))) (== "/Game/Blueprints/LevelStuff/BP_LockedDoor.BP_LockedDoor_C" (Utilities|GetClass (Variables|Default|GetNewVar_0))) (== "/Game/Blueprints/LevelStuff/BP_MovingPlatform.BP_MovingPlatform_C" (Utilities|GetClass (Variables|Default|GetNewVar_0))))
              (bind _filteredarray (Utilities|Array|FilterArray (Variables|Default|GetInteractables) "/Game/Blueprints/Interactables/BP_Shield.BP_Shield_C"))
              (if (!= (Utilities|Array|Length _filteredarray) 0)
                ;;[1 1 1] Shield Trigger
                (Actor|DestroyActor (Variables|Default|GetNewVar_0))
                (Default|CallEventDestroyedPlatform)
                (CallFunction|RemoveInteractable (.AsBP%20Shield (Utilities|Casting|CastToBP_Shield (Utilities|Array|Get(acopy) _filteredarray))))
                (bind _returnvalue_8 (Audio|SpawnSound2D "/Engine/VREditor/Sounds/UI/Floating_UI_Close.Floating_UI_Close" 1.0 1.0 0.0 0))
                (Audio|Components|Audio|Play _returnvalue_8 0.0)
                (else
                  (goto _label)))
              (else
                (goto _label)))
            (else
              ;[1 1 1] Camera
              (if (Variables|Default|GetInfinity%20Mode)
                (if (Variables|Default|GetTeleporting)
                  (Transformation|SetWorldLocation _sideviewcameracomponent (Math|Vector|MakeVector 0.0 5e+02 (Math|Float|Clamp(Float) (Variables|Default|GetNewVar_4) 5e+02 1e+07)) false true)
                  (else
                    (Transformation|SetWorldLocation _sideviewcameracomponent (Math|Vector|MakeVector 0.0 5e+02 (Math|Float|Clamp(Float) (.Z (Math|Vector|BreakVector (Transformation|GetActorLocation self))) 5e+02 1e+07)) false true)))
                (elif (Variables|Default|GetTeleporting)
                  (Transformation|SetWorldLocation _sideviewcameracomponent_2 (Math|Vector|MakeVector 0.0 5e+02 (Math|Float|Clamp(Float) (Variables|Default|GetNewVar_4) 5e+02 2.2e+03)) false true)
                  (else
                    (Transformation|SetWorldLocation _sideviewcameracomponent_2 (Math|Vector|MakeVector 0.0 5e+02 (Math|Float|Clamp(Float) (.Z (Math|Vector|BreakVector (Transformation|GetActorLocation self))) 5e+02 2.2e+03)) false true)))))))))))

(event Input|AxisEvents|InputAxisMoveRight
  (params (AxisValue :type Float%20%28single-precision%29))
  (bind _returnvalue (Utilities|Time|GetWorldDeltaSeconds))
  (bind _rotspeed (Variables|Default|GetRotSpeed))
  (bind _returnvalue_2 (* AxisValue _rotspeed _returnvalue 5e+01))
  (bind _returnvalue_3 (* _returnvalue_2 -1.0))
  ;[1 1 1] Movement
  (Utilities|FlowControl|Gate true
    (:Exit
      (Variables|Default|SetLook (Math|Vector|RotateVectorAroundAxis (Variables|Default|GetLook) _returnvalue_2 "0,1.000000, 0"))
      (if (Variables|SkinSettings|GetRotateHead)
        (Transformation|AddWorldRotation (Variables|Default|GetPaperSprite) (Math|Rotator|MakeRotator 0.0 _returnvalue_3 0.0) false false))
      (if (Variables|SkinSettings|GetRotateTrail)
        (for (_array_element _array_index) (Variables|Default|GetTrail)
          (switch int (Math|Integer|%(Integer) _array_index 2)
            (:0
              (Class|Actor|AddActorWorldRotation _array_element (Math|Rotator|MakeRotator 0.0 _returnvalue_3 0.0)))
            (:1
              (Class|Actor|AddActorWorldRotation _array_element (Math|Rotator|MakeRotator 0.0 _returnvalue_2 0.0)))))))))

(fn ConstructionScript)

(fn AddInteractable
  (params (NewItem :type BP%20Interactable%20Object%20Reference%20%28by%20ref%29))
  (bind _returnvalue (Utilities|GetClass NewItem))
  (bind _interactables (Variables|Default|GetInteractables))
  (if (== _returnvalue "/Game/Blueprints/Interactables/BP_Shield.BP_Shield_C")
    (Default|CallEventShieldPickup))
  (if (== _returnvalue "/Game/Blueprints/Interactables/BP_Star.BP_Star_C")
    (Default|CallEventStarsPickedUp)
    (else
      (Default|CallEventBoostPickup)))
  (if (Variables|/Game/Blueprints/Interactables/BP_Interactable.BP_Interactable_C|GetAttaches NewItem)
    (Utilities|Array|AddUnique (Variables|Default|GetInteractables) NewItem)
    (Components|Activation|SetActive (Variables|/Game/Blueprints/Interactables/BP_Interactable.BP_Interactable_C|GetParticleSystem NewItem) true false)
    (Components|Activation|SetActive (Variables|/Game/Blueprints/Interactables/BP_Interactable.BP_Interactable_C|GetBox NewItem) false false)
    (for (_array_element _array_index) _interactables
      (Transformation|SetActorLocation _array_element (+ (Transformation|GetActorLocation self) (Math|Vector|RotateVectorAroundAxis "0, 0,350.000000" (* _array_index (/ 3.6e+02 (Math|Conversions|ToFloat(Integer) (Utilities|Array|Length _interactables)))) "0,1.000000, 0")) false true))
    (if (== (Utilities|GetClass NewItem) "/Game/Blueprints/Interactables/BP_Shield.BP_Shield_C")
      (bind _array_element_2 (Utilities|Array|ForEachLoopwithBreak (Variables|Default|GetInteractables))
        (:LoopBody
          (if (and (== (Utilities|GetClass _array_element_2) "/Game/Blueprints/Interactables/BP_Shield.BP_Shield_C") (!= _array_element_2 NewItem))
            (return)))
        (:Completed
          (bind _returnvalue_2 (Effects|SpawnEmitterAttached "/Game/Effects/Effects/FX_Ability/Defense/P_Shield_Sphere_Buff.P_Shield_Sphere_Buff" (Variables|Collision|GetCapsuleComponent) "None" "0, 0,-10.000000" "0, 0, 0" "1.500000,1.500000,1.500000"))
          (Variables|Default|SetShield _returnvalue_2))))))

(fn RemoveInteractable
  (params (item :type BP%20Interactable%20Object%20Reference))
  (bind _interactables (Variables|Default|GetInteractables))
  (bind _returnvalue (Utilities|Array|RemoveItem (Variables|Default|GetInteractables) item))
  (if _returnvalue
    (Actor|DestroyActor item)
    (for (_array_element _array_index) _interactables
      (Transformation|SetActorLocation _array_element (+ (Transformation|GetActorLocation self) (Math|Vector|RotateVectorAroundAxis "0, 0,350.000000" (* _array_index (/ 3.6e+02 (Math|Conversions|ToFloat(Integer) (Utilities|Array|Length _interactables)))) "0,1.000000, 0")) false true))
    (if (== (Utilities|GetClass item) "/Game/Blueprints/Interactables/BP_Shield.BP_Shield_C")
      (bind _array_element_2 (Utilities|Array|ForEachLoopwithBreak _interactables)
        (:LoopBody
          (if (== (Utilities|GetClass _array_element_2) "/Game/Blueprints/Interactables/BP_Shield.BP_Shield_C")
            (return)))
        (:Completed
          (Components|DestroyComponent (Variables|Default|GetShield)))))))

(fn AnimAchievement
  (params (Achievement :type ST%20Achievement%20Structure))
  (bind _returnvalue (UserInterface|CreateWidget "/Game/Blueprints/Widgets/StandartMode/W_AchievementGet.W_AchievementGet_C" (Game|GetPlayerController 0) Achievement))
  (UserInterface|Viewport|AddtoViewport _returnvalue 0))