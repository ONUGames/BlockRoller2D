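; BP_InfoObj is an interactable that shows an info message once picked.
; Its Picked event pauses the game, opens a W_Info widget with the object's Text and destroys the actor.
; The construction script loads the BP_SaveLevel save slot named after the current level and removes the object if that level already has stars, so the info only appears until then.
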(event EventPicked
  (Game|SetGamePaused true)
  (bind _returnvalue (UserInterface|CreateWidget "/Game/Blueprints/Widgets/StandartMode/W_Info.W_Info_C" (Game|GetPlayerController 0) (Variables|Default|GetText)))
  (UserInterface|Viewport|AddtoViewport _returnvalue 0)
  (Actor|DestroyActor))

(fn ConstructionScript
  (|CallParentFunction)
  (bind _returnvalue (Game|GetCurrentLevelName true))
  (bind _returnvalue_2 (SaveGame|DoesSaveGameExist _returnvalue))
  (if _returnvalue_2
    (bind _returnvalue_3 (SaveGame|LoadGamefromSlot _returnvalue))
    (if (> (Variables|/Game/Blueprints/BP_SaveLevel.BP_SaveLevel_C|GetStars (.AsBP%20Save%20Level (Utilities|Casting|CastToBP_SaveLevel _returnvalue_3))) 0)
      (Actor|DestroyActor))))