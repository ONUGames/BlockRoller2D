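; Base pickup interactable with an empty Picked hook, triggered once when the main character overlaps its box.
; A timeline animates the sprite's scale from BeginPlay.
; Pickup calls Picked and plays a random click sound, first registering with the character if Attaches is set.
; Attaching instances parented to BP_StandartSection, flagged by the construction script, instead spawn a standalone copy of their class and destroy themselves.
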(event OnComponentBeginOverlap(Box)
  (params (OverlappedComponent :type Primitive%20Component%20Object%20Reference) (OtherActor :type Actor%20Object%20Reference) (OtherComp :type Primitive%20Component%20Object%20Reference) (OtherBodyIndex :type Integer) (bFromSweep :type Boolean) (SweepResult :type Hit%20Result%20Structure%20%28by%20ref%29))
  (bind _self self)
  (bind _outactors (Actor|GetAllActorsOfClass "/Game/Blueprints/Characters/BP_Character_Main.BP_Character_Main_C"))
  (if (== OtherActor (Utilities|Array|Get(acopy) _outactors))
    (Utilities|FlowControl|DoOnce false
      (:Completed
        (if (Variables|Default|GetAttaches)
          (bind _outactors_2 (Actor|GetAllActorsOfClass "/Game/Blueprints/Characters/BP_Character_Main.BP_Character_Main_C"))
          (if (Variables|Default|GetCreateOneMore)
            (Game|SpawnActorfromClass (Utilities|GetClass _self) (Transformation|GetActorTransform _self) "Undefined" 0 0)
            (Actor|DestroyActor)
            (else
              (Default|AddInteractable (Utilities|Array|Get(acopy) _outactors_2) self)
              (CallFunction|Picked :!label _label)
              (switch int (Math|Random|RandomIntegerinRange 0 2)
                (:0
                  (bind _returnvalue (Audio|CreateSound2D "/Engine/VREditor/Sounds/VR_click1.VR_click1" 1.0 1.0 0.0 0))
                  (Audio|Components|Audio|Play _returnvalue 0.0))
                (:1
                  (bind _returnvalue_2 (Audio|CreateSound2D "/Engine/VREditor/Sounds/VR_click2.VR_click2" 1.0 1.0 0.0 0))
                  (Audio|Components|Audio|Play _returnvalue_2 0.0))
                (:2
                  (bind _returnvalue_3 (Audio|CreateSound2D "/Engine/VREditor/Sounds/VR_click3.VR_click3" 1.0 1.0 0.0 0))
                  (Audio|Components|Audio|Play _returnvalue_3 0.0)))))
          (else
            (goto _label)))))))

(event EventBeginPlay
  (Utilities|FlowControl|Sequence
    (:then_1
      (bind _newtrack_0 (Timeline|Timeline_0 Play)
        (:Update
          (Transformation|SetWorldScale3D (Variables|Default|GetPaperSprite) (Math|Vector|MakeVector _newtrack_0 _newtrack_0 _newtrack_0)))))))

(fn ConstructionScript
  (Utilities|Casting|CastToBP_StandartSection (Actor|GetParentActor)
    (:then
      (Variables|Default|SetCreateOneMore true))
    (:CastFailed
      (Variables|Default|SetCreateOneMore false))))

(fn Picked)