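; BP_BuffSpeed is a speed buff interactable that boosts the main character's Speed when picked.
; Picked multiplies Speed on the first BP_Character_Main found, then checks its Interactables for a BP_Slow.
; If one exists, both effects are removed with a sound and the multiplier is not reverted here.
; Otherwise, after a delay, a still-valid buff removes itself and divides Speed back.
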(event Collision|EventActorBeginOverlap
  (params (OtherActor :type Actor%20Object%20Reference)))

(event EventTick
  (params (DeltaSeconds :type Float%20%28single-precision%29)))

(event EventPicked
  (bind _self self)
  (bind _outactors (Actor|GetAllActorsOfClass "/Game/Blueprints/Characters/BP_Character_Main.BP_Character_Main_C"))
  (Variables|/Game/Blueprints/Characters/BP_Character_Main.BP_Character_Main_C|SetSpeed (Utilities|Array|Get(acopy) _outactors) (* (Variables|/Game/Blueprints/Characters/BP_Character_Main.BP_Character_Main_C|GetSpeed (Utilities|Array|Get(acopy) _outactors)) 1.4))
  (bind _filteredarray (Utilities|Array|FilterArray (Variables|/Game/Blueprints/Characters/BP_Character_Main.BP_Character_Main_C|GetInteractables (Utilities|Array|Get(acopy) _outactors)) "/Game/Blueprints/Interactables/BP_Slow.BP_Slow_C"))
  (if (!= (Utilities|Array|Length _filteredarray) 0)
    (Default|RemoveInteractable (Utilities|Array|Get(acopy) _outactors) (.AsBP%20Interactable (Utilities|Casting|CastToBP_Interactable (Utilities|Array|Get(acopy) _filteredarray))))
    (Default|RemoveInteractable (Utilities|Array|Get(acopy) _outactors) self)
    (bind _returnvalue (Audio|SpawnSound2D "/Engine/VREditor/Sounds/UI/Floating_UI_Close.Floating_UI_Close" 1.0 1.0 0.0 0))
    (Audio|Components|Audio|Play _returnvalue 0.0)
    (else
      (Utilities|FlowControl|Delay 1e+01)
      (Utilities|IsValid _self
        (:Is%20Valid
          (Default|RemoveInteractable (Utilities|Array|Get(acopy) _outactors) _self)
          (Variables|/Game/Blueprints/Characters/BP_Character_Main.BP_Character_Main_C|SetSpeed (Utilities|Array|Get(acopy) _outactors) (/ (Variables|/Game/Blueprints/Characters/BP_Character_Main.BP_Character_Main_C|GetSpeed (Utilities|Array|Get(acopy) _outactors)) 1.4)))))))

(fn ConstructionScript)