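; BP_Slow is a pickup interactable that slows the main character when picked.
; Its Picked event finds the first BP_Character_Main and divides its Speed by a fixed factor.
; It then searches that character's Interactables for a BP_BuffSpeed; if one exists, it plays a UI close sound and calls TerminalDeath on both that buff and itself, so the two cancel out.
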(event EventPicked
  (bind _outactors (Actor|GetAllActorsOfClass "/Game/Blueprints/Characters/BP_Character_Main.BP_Character_Main_C"))
  (Variables|/Game/Blueprints/Characters/BP_Character_Main.BP_Character_Main_C|SetSpeed (Utilities|Array|Get(acopy) _outactors) (/ (Variables|/Game/Blueprints/Characters/BP_Character_Main.BP_Character_Main_C|GetSpeed (Utilities|Array|Get(acopy) _outactors)) 1.4))
  (bind _filteredarray (Utilities|Array|FilterArray (Variables|/Game/Blueprints/Characters/BP_Character_Main.BP_Character_Main_C|GetInteractables (Utilities|Array|Get(acopy) _outactors)) "/Game/Blueprints/Interactables/BP_BuffSpeed.BP_BuffSpeed_C"))
  (if (!= (Utilities|Array|Length _filteredarray) 0)
    (bind _returnvalue (Audio|SpawnSound2D "/Engine/VREditor/Sounds/UI/Floating_UI_Close.Floating_UI_Close" 1.0 1.0 0.0 0))
    (Audio|Components|Audio|Play _returnvalue 0.0)
    (Default|TerminalDeath (.AsBP%20Interactable (Utilities|Casting|CastToBP_Interactable (Utilities|Array|Get(acopy) _filteredarray))))
    (CallFunction|TerminalDeath)))

(fn ConstructionScript
  (|CallParentFunction))