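; BP_Key is a colour-coded key pickup that removes the locked doors sharing its number.
; Its Num value sets the cube sprite's colour, applied both in the construction script and at BeginPlay, and Tick spins the sprite around its pitch axis.
; The Picked event searches all BP_LockedDoor actors, destroys every one with a matching Num, then destroys the key itself.
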(event EventBeginPlay
  (bind _cubesprite (Variables|Default|GetCubeSprite))
  (switch int (Variables|Default|GetNum)
    (:0
      (Sprite|SetSpriteColor _cubesprite "(R=1.000000,G=0.000000,B=1.000000,A=1.000000)"))
    (:1
      (Sprite|SetSpriteColor _cubesprite "(R=0.000000,G=0.776506,B=1.000000,A=1.000000)"))
    (:2
      (Sprite|SetSpriteColor _cubesprite "(R=0.000000,G=1.000000,B=0.000000,A=1.000000)"))
    (:3
      (Sprite|SetSpriteColor _cubesprite "(R=1.000000,G=0.048928,B=0.000000,A=1.000000)"))
    (:4
      (Sprite|SetSpriteColor _cubesprite "(R=1.000000,G=1.000000,B=0.000000,A=1.000000)"))))

(event EventTick
  (params (DeltaSeconds :type Float%20%28single-precision%29))
  (Transformation|AddWorldRotation (Variables|Default|GetCubeSprite) (Math|Rotator|MakeRotator 0.0 (* DeltaSeconds 5e+01) 0.0) false false))

(event EventPicked
  (bind _outactors (Actor|GetAllActorsOfClass "/Game/Blueprints/LevelStuff/BP_LockedDoor.BP_LockedDoor_C"))
  (for _array_element _outactors
    (if (== (Variables|/Game/Blueprints/LevelStuff/BP_LockedDoor.BP_LockedDoor_C|GetNum _array_element) (Variables|Default|GetNum))
      (Actor|DestroyActor _array_element)))
  (Actor|DestroyActor))

(fn ConstructionScript
  (bind _cubesprite (Variables|Default|GetCubeSprite))
  (switch int (Variables|Default|GetNum)
    (:0
      (Sprite|SetSpriteColor _cubesprite "(R=1.000000,G=0.000000,B=1.000000,A=1.000000)"))
    (:1
      (Sprite|SetSpriteColor _cubesprite "(R=0.000000,G=0.776506,B=1.000000,A=1.000000)"))
    (:2
      (Sprite|SetSpriteColor _cubesprite "(R=0.000000,G=1.000000,B=0.000000,A=1.000000)"))
    (:3
      (Sprite|SetSpriteColor _cubesprite "(R=1.000000,G=0.048928,B=0.000000,A=1.000000)"))
    (:4
      (Sprite|SetSpriteColor _cubesprite "(R=1.000000,G=1.000000,B=0.000000,A=1.000000)"))))