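; BP_Invis is an interactable that briefly hides the main 2D character when picked.
; Picked finds the first BP_Character_Main, saves its Y position, shifts it to a fixed Y offset and hides its Paper sprite.
; After a short delay it restores Y and visibility, then removes itself from the character's interactables, with sounds bracketing the effect.
; The sprite colour is also saved but never used.
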(event EventPicked
  (bind _returnvalue (Audio|SpawnSound2D "/Engine/VREditor/Sounds/UI/Dockable_Window_Open.Dockable_Window_Open" 1.0 1.0 0.0 0))
  (Audio|Components|Audio|Play _returnvalue 0.0)
  (bind _outactors (Actor|GetAllActorsOfClass "/Game/Blueprints/Characters/BP_Character_Main.BP_Character_Main_C"))
  (Variables|Default|SetNewVar_0 (.Y (Math|Vector|BreakVector (Transformation|GetActorLocation (Utilities|Array|Get(acopy) _outactors)))))
  (Transformation|SetActorLocation (Utilities|Array|Get(acopy) _outactors) (Math|Vector|MakeVector (.X (Math|Vector|BreakVector (Transformation|GetActorLocation (Utilities|Array|Get(acopy) _outactors)))) 2e+02 (.Z (Math|Vector|BreakVector (Transformation|GetActorLocation (Utilities|Array|Get(acopy) _outactors))))) false false)
  (Variables|Default|SetNewVar_1 (Variables|/Script/Paper2D.PaperSpriteComponent|GetSpriteColor (Variables|/Game/Blueprints/Characters/BP_Character_Main.BP_Character_Main_C|GetPaperSprite (Utilities|Array|Get(acopy) _outactors))))
  (Rendering|SetVisibility (Variables|/Game/Blueprints/Characters/BP_Character_Main.BP_Character_Main_C|GetPaperSprite (Utilities|Array|Get(acopy) _outactors)) false false)
  (Utilities|FlowControl|Delay 2.0)
  (Transformation|SetActorLocation (Utilities|Array|Get(acopy) _outactors) (Math|Vector|MakeVector (.X (Math|Vector|BreakVector (Transformation|GetActorLocation (Utilities|Array|Get(acopy) _outactors)))) (Variables|Default|GetNewVar_0) (.Z (Math|Vector|BreakVector (Transformation|GetActorLocation (Utilities|Array|Get(acopy) _outactors))))) false false)
  (Rendering|SetVisibility (Variables|/Game/Blueprints/Characters/BP_Character_Main.BP_Character_Main_C|GetPaperSprite (Utilities|Array|Get(acopy) _outactors)) true false)
  (Default|RemoveInteractable (Utilities|Array|Get(acopy) _outactors) self)
  (bind _returnvalue_2 (Audio|SpawnSound2D "/Engine/VREditor/Sounds/UI/Dockable_Window_Close.Dockable_Window_Close" 1.0 1.0 0.0 0))
  (Audio|Components|Audio|Play _returnvalue_2 0.0))

(fn ConstructionScript
  (|CallParentFunction))