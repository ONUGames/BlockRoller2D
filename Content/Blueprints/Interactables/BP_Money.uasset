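; Money pickup interactable that appears only occasionally and adds currency to the player's global save.
; On BeginPlay it runs the parent logic, then destroys itself unless a one-in-twenty random roll succeeds, so most placed instances vanish.
; The Picked event adds a fixed amount to Money in the global save, writes the save immediately and destroys the actor.
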(event EventBeginPlay
  (|CallParentFunction)
  (if (not (== (Math|Random|RandomIntegerinRange 1 20) 1))
    (Actor|DestroyActor)))

(event EventPicked
  (bind _asbp_global_save (CallFunction|GetGlobalSave))
  (Variables|/Game/Blueprints/BP_GlobalSave.BP_GlobalSave_C|SetMoney _asbp_global_save (+ (Variables|/Game/Blueprints/BP_GlobalSave.BP_GlobalSave_C|GetMoney _asbp_global_save) 20))
  (CallFunction|SaveGlobal _asbp_global_save)
  (Actor|DestroyActor))

(fn ConstructionScript
  (|CallParentFunction))