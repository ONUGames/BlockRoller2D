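; Level-building actor that creates a horizontal row of platforms with a random gap.
; On BeginPlay it spawns six evenly spaced BP_Platform actors along X from its own location and stores them in Platforms.
; It drops one random array entry without destroying that actor, then destroys a random remaining platform.
; The construction script separately hides one of six Paper sprites at random, independent of the runtime gap.
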(event EventBeginPlay
  (bind _self self)
  (bind _platforms (Variables|Default|GetPlatforms))
  (bind _returnvalue (Utilities|Array|Length _platforms))
  (bind _returnvalue_2 (Transformation|GetActorLocation _self))
  (bind _returnvalue_3 (- _returnvalue 1))
  (bind (_x _y _z) (Math|Vector|BreakVector _returnvalue_2))
  (bind _returnvalue_4 (Math|Random|RandomIntegerinRange 0 _returnvalue_3))
  (for _index (range 1 6)
    (bind _returnvalue_5 (Game|SpawnActorfromClass "/Game/Blueprints/LevelStuff/BP_Platform.BP_Platform_C" (Math|Transform|MakeTransform (Math|Vector|MakeVector (+ (* (+ _index -1) 3.3e+02) _x) 0.0 _z)) "Undefined" self 0))
    (Utilities|Array|Add (Variables|Default|GetPlatforms) _returnvalue_5))
  (Utilities|Array|RemoveIndex _platforms _returnvalue_4)
  (Actor|DestroyActor (Utilities|Array|Get(acopy) _platforms _returnvalue_4)))

(fn ConstructionScript
  (switch int (Math|Random|RandomIntegerinRange 0 5)
    (:0
      (Rendering|SetVisibility (Variables|Default|GetPaperSprite5) false false))
    (:1
      (Rendering|SetVisibility (Variables|Default|GetPaperSprite4) false false))
    (:2
      (Rendering|SetVisibility (Variables|Default|GetPaperSprite3) false false))
    (:3
      (Rendering|SetVisibility (Variables|Default|GetPaperSprite2) false false))
    (:4
      (Rendering|SetVisibility (Variables|Default|GetPaperSprite1) false false))
    (:5
      (Rendering|SetVisibility (Variables|Default|GetPaperSprite) false false))))