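; BP_Platform is a level platform Blueprint whose ledge takes on a look that matches the current level.
; On BeginPlay it checks the current level name for IceHill, LavaLake or NeonHell and swaps the Ledge component's sprite to that theme's sprite.
; Levels matching none of these keep the default sprite, and the construction script is empty.
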(event EventBeginPlay
  (bind _ledge (Variables|Default|GetLedge))
  (bind _returnvalue (Game|GetCurrentLevelName true))
  (if (Utilities|String|Contains _returnvalue "IceHill")
    (Rendering|Components|Sprite|SetSprite _ledge "/Game/2DSideScroller/Sprites/bluebar_Sprite.bluebar_Sprite")
    (elif (Utilities|String|Contains _returnvalue "LavaLake")
      (Rendering|Components|Sprite|SetSprite _ledge "/Game/2DSideScroller/Sprites/redplatform_Sprite.redplatform_Sprite")
      (elif (Utilities|String|Contains _returnvalue "NeonHell")
        (Rendering|Components|Sprite|SetSprite _ledge "/Game/2DSideScroller/Sprites/rose_Sprite.rose_Sprite")))))

(fn ConstructionScript)