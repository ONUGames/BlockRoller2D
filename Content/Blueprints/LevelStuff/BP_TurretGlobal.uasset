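; BP_TurretGlobal is a Paper2D turret that fires BP_Projectile actors at the main character while it is within range.
; Tick orbits two sprites around the Y axis, looks up the player, and shoots either single shots or three-projectile shotgun fans.
; Delay nodes in Tick throttle the fire rate and handle reloading once ammo runs out, with each volley costing one round.
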(event EventTick
  (params (DeltaSeconds :type Float%20%28single-precision%29))
  (bind _returnvalue (Transformation|GetActorLocation))
  (bind _self self)
  (bind _self_2 self)
  (bind _projectile_speed (Variables|Public|GetProjectile%20Speed))
  (bind _returnvalue_2 (Transformation|GetActorTransform _self))
  (CallFunction|SetTurretRotation (* DeltaSeconds 1.3e+02))
  (Utilities|FlowControl|Sequence
    (:then_0
      (bind _outactors (Actor|GetAllActorsOfClass "/Game/Blueprints/Characters/BP_Character_Main.BP_Character_Main_C"))
      (if (Variables|Public|GetShotgun)
        (if (and (<= (Math|Vector|VectorLength (- _returnvalue (Transformation|GetActorLocation (Utilities|Array|Get(acopy) _outactors)))) (Variables|Public|GetRange)) (> (Variables|Default|GetAmmo) 0))
          (Utilities|FlowControl|Delay (/ 1.0 (Variables|Public|GetShots%20Per%20Second)))
          (Math|Integer|DecrementInt (Variables|Default|GetAmmo)
            (:%20%20
              (Game|SpawnActorfromClass "/Game/Blueprints/LevelStuff/BP_Projectile.BP_Projectile_C" _returnvalue_2 "Undefined" _self (- (Transformation|GetActorLocation (Utilities|Array|Get(acopy) _outactors)) _returnvalue) _projectile_speed 0)
              (Game|SpawnActorfromClass "/Game/Blueprints/LevelStuff/BP_Projectile.BP_Projectile_C" _returnvalue_2 "Undefined" _self (Math|Vector|RotateVectorAroundAxis (- (Transformation|GetActorLocation (Utilities|Array|Get(acopy) _outactors)) _returnvalue) 15.0 "0,1.000000, 0") _projectile_speed 0)
              (Game|SpawnActorfromClass "/Game/Blueprints/LevelStuff/BP_Projectile.BP_Projectile_C" _returnvalue_2 "Undefined" _self (Math|Vector|RotateVectorAroundAxis (- (Transformation|GetActorLocation (Utilities|Array|Get(acopy) _outactors)) _returnvalue) -15.0 "0,1.000000, 0") _projectile_speed 0))))
        (elif (and (<= (Math|Vector|VectorLength (- _returnvalue (Transformation|GetActorLocation (Utilities|Array|Get(acopy) _outactors)))) (Variables|Public|GetRange)) (> (Variables|Default|GetAmmo) 0))
          (Utilities|FlowControl|Delay (/ 1.0 (Variables|Public|GetShots%20Per%20Second)))
          (Game|SpawnActorfromClass "/Game/Blueprints/LevelStuff/BP_Projectile.BP_Projectile_C" (Transformation|GetActorTransform _self_2) "Undefined" _self_2 (- (Transformation|GetActorLocation (Utilities|Array|Get(acopy) _outactors)) _returnvalue) (Variables|Public|GetProjectile%20Speed) 0)
          (Math|Integer|DecrementInt (Variables|Default|GetAmmo)))))
    (:then_1
      (if (<= (Variables|Default|GetAmmo) 0)
        (Utilities|FlowControl|Delay (Variables|Public|GetReload%20Time))
        (Variables|Default|SetAmmo (Variables|Public|GetAmmo%20Per%20Load))))))

(fn ConstructionScript
  (Variables|Default|SetAmmo (Variables|Public|GetAmmo%20Per%20Load)))

(fn SetTurretRotation
  (params (Rotation :type Float%20%28single-precision%29))
  (bind _papersprite1 (Variables|Default|GetPaperSprite1))
  (bind _papersprite (Variables|Default|GetPaperSprite))
  (Variables|Default|SetRotation (Math|Float|%(Float) Rotation 3.6e+02))
  (Transformation|SetRelativeLocation _papersprite (Math|Vector|RotateVectorAroundAxis (Variables|/Script/Engine.SceneComponent|GetRelativeLocation _papersprite) Rotation "0,1.000000, 0") false false)
  (Transformation|SetRelativeLocation _papersprite1 (Math|Vector|RotateVectorAroundAxis (Variables|/Script/Engine.SceneComponent|GetRelativeLocation _papersprite1) Rotation "0,1.000000, 0") false false))