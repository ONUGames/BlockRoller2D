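; Moving platform that circles in the vertical XZ plane and carries settings for a nested BP_CirclePlatform child actor.
; After a short or long start delay, a gate lets Tick advance the angle by Speed and place the platform at Radius.
; The construction script previews radius, start position and angle via sphere and arrow, then pushes the child radius, speed and offset into the child actor and updates its preview.
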(event EventBeginPlay
  (if (CallFunction|IsDelayLong)
    (Utilities|FlowControl|Delay 4.0)
    (Utilities|FlowControl|Gate true) ; enters at Open
    (else
      (Utilities|FlowControl|Delay 1.0)
      (Utilities|FlowControl|Gate true) ; enters at Open
    )))

(event EventTick
  (params (DeltaSeconds :type Float%20%28single-precision%29))
  (Utilities|FlowControl|Gate true
    (:Exit
      (Variables|Default|SetOffset (Math|Float|%(Float) (+ (* DeltaSeconds (Variables|Default|GetSpeed)) (Variables|Default|GetOffset)) 3.6e+02))
      (Transformation|SetRelativeLocation (Variables|Default|GetBP_Platform) (Math|Vector|RotateVectorAroundAxis (Math|Vector|MakeVector (Variables|Default|GetRadius) 0.0 0.0) (Variables|Default|GetOffset) "0,-1.000000, 0") false false))))

(fn ConstructionScript
  (bind _radius_child (Variables|Default|GetRadius_Child))
  (Components|Sphere|SetSphereRadius (Variables|Default|GetSphere) (Variables|Default|GetRadius) true)
  (Transformation|AddLocalOffset (Variables|Default|GetBP_Platform) (Math|Vector|RotateVectorAroundAxis (Math|Vector|MakeVector (Variables|Default|GetRadius) 0.0 0.0) (Variables|Default|GetOffset) "0,-1.000000, 0") false false)
  (Transformation|SetRelativeRotation (Variables|Default|GetArrow) (Math|Rotator|MakeRotator 0.0 (Variables|Default|GetOffset) 0.0) false false)
  (bind _asbp_circle_platform (Utilities|Casting|CastToBP_CirclePlatform (Variables|/Script/Engine.ChildActorComponent|GetChildActor (Variables|Default|GetBP_CirclePlatform))))
  (Variables|/Game/Blueprints/LevelStuff/BP_CirclePlatform.BP_CirclePlatform_C|SetRadius _asbp_circle_platform _radius_child)
  (Variables|/Game/Blueprints/LevelStuff/BP_CirclePlatform.BP_CirclePlatform_C|SetSpeed _asbp_circle_platform (Variables|Default|GetSpeed_Child))
  (Variables|/Game/Blueprints/LevelStuff/BP_CirclePlatform.BP_CirclePlatform_C|SetOffset _asbp_circle_platform (Variables|Default|GetOffset_Child))
  (Components|Sphere|SetSphereRadius (Variables|/Game/Blueprints/LevelStuff/BP_CirclePlatform.BP_CirclePlatform_C|GetSphere _asbp_circle_platform) _radius_child true)
  (Transformation|SetRelativeLocation (Variables|/Game/Blueprints/LevelStuff/BP_CirclePlatform.BP_CirclePlatform_C|GetBP_Platform _asbp_circle_platform) (Math|Vector|RotateVectorAroundAxis (Math|Vector|MakeVector (Variables|/Game/Blueprints/LevelStuff/BP_CirclePlatform.BP_CirclePlatform_C|GetRadius _asbp_circle_platform) 0.0 0.0) (Variables|/Game/Blueprints/LevelStuff/BP_CirclePlatform.BP_CirclePlatform_C|GetOffset _asbp_circle_platform) "0,-1.000000, 0") false false)
  (Transformation|SetRelativeRotation (Variables|/Game/Blueprints/LevelStuff/BP_CirclePlatform.BP_CirclePlatform_C|GetArrow _asbp_circle_platform) (Math|Rotator|MakeRotator 0.0 (Variables|/Game/Blueprints/LevelStuff/BP_CirclePlatform.BP_CirclePlatform_C|GetOffset _asbp_circle_platform) 0.0) false false))