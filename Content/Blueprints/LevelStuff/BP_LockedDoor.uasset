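; BP_LockedDoor is a color-coded locked door that absorbs projectiles; this Blueprint contains no unlock logic.
; The Num value selects the CubeSprite tint, set in both the Construction Script and BeginPlay.
; Tick steadily spins the sprite around its pitch axis.
; When a BP_Projectile of that exact class overlaps the Box, the door destroys it and plays the Laser_Push sound in 2D.
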(event OnComponentBeginOverlap(Box)
  (params (OverlappedComponent :type Primitive%20Component%20Object%20Reference) (OtherActor :type Actor%20Object%20Reference) (OtherComp :type Primitive%20Component%20Object%20Reference) (OtherBodyIndex :type Integer) (bFromSweep :type Boolean) (SweepResult :type Hit%20Result%20Structure%20%28by%20ref%29))
  (if (== (Utilities|GetClass OtherActor) "/Game/Blueprints/LevelStuff/BP_Projectile.BP_Projectile_C")
    (Actor|DestroyActor OtherActor)
    (bind _returnvalue (Audio|CreateSound2D "/Engine/VREditor/Sounds/UI/Laser_Push.Laser_Push" 1.0 1.0 0.0 0))
    (Audio|Components|Audio|Play _returnvalue 0.0)))

(event EventBeginPlay
  (bind _cubesprite (Variables|Default|GetCubeSprite))
  (switch int (Variables|Default|GetNum)
    (:0
      (Sprite|SetSpriteColor _cubesprite "(R=1.000000,G=0.000000,B=1.000000,A=1.000000)"))
    (:1
      (Sprite|SetSpriteColor _cubesprite "(R=0.000000,G=0.776506,B=1.000000,A=1.000000)"))
    (:2
      (Sprite|SetSpriteColor _cubesprite "(R=0.000000,G=1.000000,B=0.000000,A=1.000000)"))
    (:3
      (Sprite|SetSpriteColor _cubesprite "(R=1.000000,G=0.048928,B=0.000000,A=1.000000)"))
    (:4
      (Sprite|SetSpriteColor _cubesprite "(R=1.000000,G=1.000000,B=0.000000,A=1.000000)"))))

(event EventTick
  (params (DeltaSeconds :type Float%20%28single-precision%29))
  (Transformation|AddWorldRotation (Variables|Default|GetCubeSprite) (Math|Rotator|MakeRotator 0.0 (* DeltaSeconds 5e+01) 0.0) false false))

(fn ConstructionScript
  (bind _cubesprite (Variables|Default|GetCubeSprite))
  (switch int (Variables|Default|GetNum)
    (:0
      (Sprite|SetSpriteColor _cubesprite "(R=1.000000,G=0.000000,B=1.000000,A=1.000000)"))
    (:1
      (Sprite|SetSpriteColor _cubesprite "(R=0.000000,G=0.776506,B=1.000000,A=1.000000)"))
    (:2
      (Sprite|SetSpriteColor _cubesprite "(R=0.000000,G=1.000000,B=0.000000,A=1.000000)"))
    (:3
      (Sprite|SetSpriteColor _cubesprite "(R=1.000000,G=0.048928,B=0.000000,A=1.000000)"))
    (:4
      (Sprite|SetSpriteColor _cubesprite "(R=1.000000,G=1.000000,B=0.000000,A=1.000000)"))))