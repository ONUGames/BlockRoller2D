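; Moving platform that travels back and forth along an angled XZ line of set Length, carrying a child BP_CirclePlatform.
; The construction script places the endpoint sprite, arrow and offset platform, and passes radius, speed and offset to the child.
; After a short or long startup delay, a gate lets Tick sweep-move the actor, flipping Speed at either end.
; A sweep starting inside the main character calls its EventHit.
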(event EventBeginPlay
  (bind _self self)
  (Variables|Default|SetDelta (+ (Variables|Default|GetMoveOffset) (Variables|Default|GetDelta)))
  (Transformation|AddLocalOffset (Variables|Default|GetBP_Platform) "0, 0, 0" false false)
  (if (CallFunction|IsDelayLong)
    (Utilities|FlowControl|Delay 4.0)
    (Utilities|FlowControl|Gate true) ; enters at Open
    (else
      (Utilities|FlowControl|Delay 1.0)
      (Utilities|FlowControl|Gate true) ; enters at Open
    )))

(event EventTick
  (params (DeltaSeconds :type Float%20%28single-precision%29))
  (bind _self self)
  (bind _speed (Variables|Default|GetSpeed))
  (bind _returnvalue (* DeltaSeconds _speed))
  (Utilities|FlowControl|Gate true
    (:Exit
      (Variables|Default|SetDelta (+ _returnvalue (Variables|Default|GetDelta)))
      (bind _sweephitresult (Transformation|SetActorLocation _self (+ (* (Math|Vector|RotateVectorAroundAxis "1.000000, 0, 0" (* (Variables|Default|GetAngle) -1.0) "0,1.000000, 0") _returnvalue) (Transformation|GetActorLocation _self)) true false))
      (bind _outactors (Actor|GetAllActorsOfClass "/Game/Blueprints/Characters/BP_Character_Main.BP_Character_Main_C"))
      (if (and (.bInitialOverlap (Collision|BreakHitResult _sweephitresult)) (== (Utilities|Array|Get(acopy) _outactors) (.HitActor (Collision|BreakHitResult _sweephitresult))))
        (Utilities|FlowControl|Sequence
          (:then_0
            (Default|EventHit (Utilities|Array|Get(acopy) _outactors) self))
          (:then_1
            (if (< (Variables|Default|GetDelta) 0.0) :!label _label
              (Variables|Default|SetDelta 0.0)
              (Math|Float|NegateFloat (Variables|Default|GetSpeed) :!label _label_2)
              (elif (> (Variables|Default|GetDelta) (Variables|Default|GetLength))
                (Variables|Default|SetDelta (Variables|Default|GetLength))
                (goto _label_2)))))
        (else
          (goto _label))))))

(fn ConstructionScript
  (bind _papersprite1 (Variables|Default|GetPaperSprite1))
  (bind _radius_child (Variables|Default|GetRadius_Child))
  (Transformation|AddLocalOffset (Variables|Default|GetPaperSprite) (* (Math|Vector|RotateVectorAroundAxis "1.000000, 0, 0" (* (Variables|Default|GetAngle) -1.0) "0,1.000000, 0") (Variables|Default|GetLength)) false false)
  (Transformation|SetWorldRotation (Variables|Default|GetArrow) (Math|Rotator|MakeRotator 0.0 (Variables|Default|GetAngle) 0.0) false false)
  (Transformation|AddLocalOffset (Variables|Default|GetBP_Platform) (* (Math|Vector|RotateVectorAroundAxis "1.000000, 0, 0" (* (Variables|Default|GetAngle) -1.0) "0,1.000000, 0") (Math|Float|Clamp(Float) (Variables|Default|GetMoveOffset) 0.0 (Variables|Default|GetLength))) false false)
  (if (== (Variables|Default|GetMoveOffset) 0.0)
    (Rendering|SetVisibility _papersprite1 false false)
    (else
      (Rendering|SetVisibility _papersprite1 true false)))
  (bind _asbp_circle_platform (Utilities|Casting|CastToBP_CirclePlatform (Variables|/Script/Engine.ChildActorComponent|GetChildActor (Variables|Default|GetBP_CirclePlatform))))
  (Variables|/Game/Blueprints/LevelStuff/BP_CirclePlatform.BP_CirclePlatform_C|SetRadius _asbp_circle_platform _radius_child)
  (Variables|/Game/Blueprints/LevelStuff/BP_CirclePlatform.BP_CirclePlatform_C|SetSpeed _asbp_circle_platform (Variables|Default|GetSpeed_Child))
  (Variables|/Game/Blueprints/LevelStuff/BP_CirclePlatform.BP_CirclePlatform_C|SetOffset _asbp_circle_platform (Variables|Default|GetOffset_Child))
  (Components|Sphere|SetSphereRadius (Variables|/Game/Blueprints/LevelStuff/BP_CirclePlatform.BP_CirclePlatform_C|GetSphere _asbp_circle_platform) _radius_child true)
  (Transformation|SetRelativeLocation (Variables|/Game/Blueprints/LevelStuff/BP_CirclePlatform.BP_CirclePlatform_C|GetBP_Platform _asbp_circle_platform) (Math|Vector|RotateVectorAroundAxis (Math|Vector|MakeVector (Variables|/Game/Blueprints/LevelStuff/BP_CirclePlatform.BP_CirclePlatform_C|GetRadius _asbp_circle_platform) 0.0 0.0) (Variables|/Game/Blueprints/LevelStuff/BP_CirclePlatform.BP_CirclePlatform_C|GetOffset _asbp_circle_platform) "0,-1.000000, 0") false false)
  (Transformation|SetRelativeRotation (Variables|/Game/Blueprints/LevelStuff/BP_CirclePlatform.BP_CirclePlatform_C|GetArrow _asbp_circle_platform) (Math|Rotator|MakeRotator 0.0 (Variables|/Game/Blueprints/LevelStuff/BP_CirclePlatform.BP_CirclePlatform_C|GetOffset _asbp_circle_platform) 0.0) false false))