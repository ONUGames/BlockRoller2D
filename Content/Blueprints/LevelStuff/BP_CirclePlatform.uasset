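; BP_CirclePlatform is a level platform that circles continuously in the vertical XZ plane around the actor.
; Tick advances Offset by Speed, wraps it at 360 degrees, then sets BPPlatform's relative location to a Radius-length vector rotated by that angle.
; The construction script sizes Sphere to Radius, offsets the platform to its starting angle and pitches Arrow to match Offset.
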(event EventTick
  (params (DeltaSeconds :type Float%20%28single-precision%29))
  (Variables|Default|SetOffset (Math|Float|%(Float) (+ (* DeltaSeconds (Variables|Default|GetSpeed)) (Variables|Default|GetOffset)) 3.6e+02))
  (Transformation|SetRelativeLocation (Variables|Default|GetBP_Platform) (Math|Vector|RotateVectorAroundAxis (Math|Vector|MakeVector (Variables|Default|GetRadius) 0.0 0.0) (Variables|Default|GetOffset) "0,-1.000000, 0") false false))

(fn ConstructionScript
  (Components|Sphere|SetSphereRadius (Variables|Default|GetSphere) (Variables|Default|GetRadius) true)
  (Transformation|AddLocalOffset (Variables|Default|GetBP_Platform) (Math|Vector|RotateVectorAroundAxis (Math|Vector|MakeVector (Variables|Default|GetRadius) 0.0 0.0) (Variables|Default|GetOffset) "0,-1.000000, 0") false false)
  (Transformation|SetRelativeRotation (Variables|Default|GetArrow) (Math|Rotator|MakeRotator 0.0 (Variables|Default|GetOffset) 0.0) false false))