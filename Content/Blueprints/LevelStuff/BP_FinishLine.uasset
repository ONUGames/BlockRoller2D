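; BP_FinishLine is a level finish trigger that ends play with a win screen when the main character enters its box.
; On overlap, a gate that closes after first use makes the sequence run once.
; It overrides the character's Look, zeroes RotSpeed and plays a success sound.
; After short delays it shows W_WinScreen with the mouse cursor, then pauses the game.
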(event OnComponentBeginOverlap(Box)
  (params (OverlappedComponent :type Primitive%20Component%20Object%20Reference) (OtherActor :type Actor%20Object%20Reference) (OtherComp :type Primitive%20Component%20Object%20Reference) (OtherBodyIndex :type Integer) (bFromSweep :type Boolean) (SweepResult :type Hit%20Result%20Structure%20%28by%20ref%29))
  (bind _returnvalue (Game|GetPlayerController 0))
  (bind _outactors (Actor|GetAllActorsOfClass "/Game/Blueprints/Characters/BP_Character_Main.BP_Character_Main_C"))
  (if (== OtherActor (Utilities|Array|Get(acopy) _outactors))
    (Utilities|FlowControl|Sequence
      (:then_0
        (Utilities|FlowControl|Gate false :!label _label
          (:Exit
            (bind _outactors_2 (Actor|GetAllActorsOfClass "/Game/Blueprints/Characters/BP_Character_Main.BP_Character_Main_C"))
            (Variables|/Game/Blueprints/Characters/BP_Character_Main.BP_Character_Main_C|SetLook (Utilities|Array|Get(acopy) _outactors_2) "0, 0,1.000000")
            (Variables|/Game/Blueprints/Characters/BP_Character_Main.BP_Character_Main_C|SetRotSpeed (Utilities|Array|Get(acopy) _outactors_2) 0.0)
            (bind _returnvalue_2 (Audio|CreateSound2D "/Engine/EditorSounds/Notifications/CompileSuccess.CompileSuccess" 1.0 1.0 0.0 0))
            (Audio|Components|Audio|Play _returnvalue_2 0.0)
            (Utilities|FlowControl|Delay 0.6)
            (bind _returnvalue_3 (UserInterface|CreateWidget "/Game/Blueprints/Widgets/StandartMode/W_WinScreen.W_WinScreen_C" _returnvalue))
            (UserInterface|Viewport|AddtoPlayerScreen _returnvalue_3)
            (Variables|/Script/Engine.PlayerController|SetbShowMouseCursor _returnvalue true)
            (Utilities|FlowControl|Delay 0.2)
            (Game|SetGamePaused true))))
      (:then_1
        (goto _label Close)))))

(fn ConstructionScript)