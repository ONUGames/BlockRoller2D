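; BP_Portal_OneTime is a single-use portal that teleports the main character to a linked portal.
; When the first BP_Character_Main found overlaps its Box and is not already Teleporting, it searches BP_Portal actors for another with the same PortalNum.
; On the first match it stops searching, calls the character's PortalTeleport with both locations, then destroys itself and the destination portal.
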(event OnComponentBeginOverlap(Box)
  (params (OverlappedComponent :type Primitive%20Component%20Object%20Reference) (OtherActor :type Actor%20Object%20Reference) (OtherComp :type Primitive%20Component%20Object%20Reference) (OtherBodyIndex :type Integer) (bFromSweep :type Boolean) (SweepResult :type Hit%20Result%20Structure%20%28by%20ref%29))
  (bind _outactors (Actor|GetAllActorsOfClass "/Game/Blueprints/Characters/BP_Character_Main.BP_Character_Main_C"))
  (if (and (== OtherActor (Utilities|Array|Get(acopy) _outactors)) (not (Variables|/Game/Blueprints/Characters/BP_Character_Main.BP_Character_Main_C|GetTeleporting (Utilities|Array|Get(acopy) _outactors))))
    (bind _outactors_2 (Actor|GetAllActorsOfClass "/Game/Blueprints/LevelStuff/BP_Portal.BP_Portal_C"))
    (bind _array_element (Utilities|Array|ForEachLoopwithBreak _outactors_2 :!label _label)
      (:LoopBody
        (if (and (== (Variables|/Game/Blueprints/LevelStuff/BP_Portal.BP_Portal_C|GetPortalNum _array_element) (Variables|Default|GetPortalNum)) (!= _array_element self))
          (Utilities|FlowControl|Sequence
            (:then_0
              (goto _label Break))
            (:then_1
              (Default|PortalTeleport (Utilities|Array|Get(acopy) _outactors) (Transformation|GetActorLocation) (Transformation|GetActorLocation _array_element))
              (Actor|DestroyActor self)
              (Actor|DestroyActor _array_element))))))))

(event EventBeginPlay
  (|CallParentFunction) ; This node is disabled and will not be called.\nDrag off pins to build functionality.
)

(event Collision|EventActorBeginOverlap
  (params (OtherActor :type Actor%20Object%20Reference)))

(event EventTick
  (params (DeltaSeconds :type Float%20%28single-precision%29))
  (|CallParentFunction DeltaSeconds) ; This node is disabled and will not be called.\nDrag off pins to build functionality.
)

(fn ConstructionScript
  (|CallParentFunction))