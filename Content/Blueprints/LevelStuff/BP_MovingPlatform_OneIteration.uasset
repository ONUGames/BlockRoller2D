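; Moving platform, apparently for a 2D side-view level, that makes a single one-way trip along an angled line and stops.
; After a start delay, Tick passes through a gate to sweep-move it by Speed, zeroing Speed once travel leaves the zero-to-Length range.
; An initial-overlap sweep hit on BP_Character_Main calls that character's EventHit.
; The construction script offsets an endpoint sprite, aims the arrow and pre-shifts the platform by MoveOffset.
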(event EventBeginPlay
  (bind _self self)
  (Variables|Default|SetDelta (+ (Variables|Default|GetMoveOffset) (Variables|Default|GetDelta)))
  (Transformation|AddLocalOffset (Variables|Default|GetBP_Platform) "0, 0, 0" false false)
  (Utilities|FlowControl|Delay (+ (Variables|Default|GetDelay) 1.0))
  (Utilities|FlowControl|Gate true) ; enters at Open
)

(event EventTick
  (params (DeltaSeconds :type Float%20%28single-precision%29))
  (bind _self self)
  (Utilities|FlowControl|Gate true
    (:Exit
      (Variables|Default|SetDelta (+ (* DeltaSeconds (Variables|Default|GetSpeed)) (Variables|Default|GetDelta)))
      (bind _sweephitresult (Transformation|SetActorLocation _self (+ (* (Math|Vector|RotateVectorAroundAxis "1.000000, 0, 0" (* (Variables|Default|GetAngle) -1.0) "0,1.000000, 0") (* DeltaSeconds (Variables|Default|GetSpeed))) (Transformation|GetActorLocation _self)) true false))
      (bind _outactors (Actor|GetAllActorsOfClass "/Game/Blueprints/Characters/BP_Character_Main.BP_Character_Main_C"))
      (if (and (.bInitialOverlap (Collision|BreakHitResult _sweephitresult)) (== (Utilities|Array|Get(acopy) _outactors) (.HitActor (Collision|BreakHitResult _sweephitresult))))
        (Utilities|FlowControl|Sequence
          (:then_0
            (Default|EventHit (Utilities|Array|Get(acopy) _outactors) self))
          (:then_1
            (if (< (Variables|Default|GetDelta) 0.0) :!label _label
              (Variables|Default|SetDelta 0.0)
              (Variables|Default|SetSpeed 0.0 :!label _label_2)
              (elif (> (Variables|Default|GetDelta) (Variables|Default|GetLength))
                (Variables|Default|SetDelta (Variables|Default|GetLength))
                (goto _label_2)))))
        (else
          (goto _label))))))

(fn ConstructionScript
  (bind _papersprite1 (Variables|Default|GetPaperSprite1))
  (Transformation|AddLocalOffset (Variables|Default|GetPaperSprite) (* (Math|Vector|RotateVectorAroundAxis "1.000000, 0, 0" (* (Variables|Default|GetAngle) -1.0) "0,1.000000, 0") (Variables|Default|GetLength)) false false)
  (Transformation|SetWorldRotation (Variables|Default|GetArrow) (Math|Rotator|MakeRotator 0.0 (Variables|Default|GetAngle) 0.0) false false)
  (Transformation|AddLocalOffset (Variables|Default|GetBP_Platform) (* (Math|Vector|RotateVectorAroundAxis "1.000000, 0, 0" (* (Variables|Default|GetAngle) -1.0) "0,1.000000, 0") (Math|Float|Clamp(Float) (Variables|Default|GetMoveOffset) 0.0 (Variables|Default|GetLength))) false false)
  (if (== (Variables|Default|GetMoveOffset) 0.0)
    (Rendering|SetVisibility _papersprite1 false false)
    (else
      (Rendering|SetVisibility _papersprite1 true false))))