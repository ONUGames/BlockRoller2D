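; BP_Trail is a sprite actor that trails behind another actor on the X/Z plane, like one segment of a follow chain.
; On begin play it stores its starting Y and applies the configured sprite and color to CubeSprite.
; Each tick, if its planar distance to ActorToFollow exceeds Distance, it teleports along the line between them to exactly that distance, keeping its original Y.
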(event EventBeginPlay
  (bind _cubesprite (Variables|Default|GetCubeSprite))
  (Variables|Default|SetNewVar_0 (.Y (Math|Vector|BreakVector (Transformation|GetActorLocation self))))
  (Rendering|Components|Sprite|SetSprite _cubesprite (Variables|Default|GetSprite))
  (Sprite|SetSpriteColor _cubesprite (Variables|Default|GetColor)))

(event EventTick
  (params (DeltaSeconds :type Float%20%28single-precision%29))
  (bind _self self)
  (bind _actortofollow (Variables|Default|GetActorToFollow))
  (bind _distance (Variables|Default|GetDistance))
  (bind _returnvalue (Transformation|GetActorLocation _actortofollow))
  (bind _returnvalue_2 (Transformation|GetActorLocation _self))
  (bind (_x _y _z) (Math|Vector|BreakVector _returnvalue_2))
  (bind (_x_2 _y_2 _z_2) (Math|Vector|BreakVector _returnvalue))
  (bind _returnvalue_3 (- _z_2 _z))
  (bind _returnvalue_4 (- _x_2 _x))
  (bind _returnvalue_5 (Math|Float|Square _returnvalue_3))
  (bind _returnvalue_6 (Math|Float|Square _returnvalue_4))
  (bind _returnvalue_7 (+ _returnvalue_6 _returnvalue_5))
  (bind _returnvalue_8 (Math|Float|Sqrt _returnvalue_7))
  (if (> _returnvalue_8 _distance)
    (Transformation|SetActorLocation self (Math|Vector|MakeVector (- _x_2 (/ (* _returnvalue_4 _distance) _returnvalue_8)) (Variables|Default|GetNewVar_0) (- _z_2 (/ (* _returnvalue_3 _distance) _returnvalue_8))) false true)))

(fn ConstructionScript)