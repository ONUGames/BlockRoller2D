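; BP_EasySection7 is an easy-difficulty level section, filed under InfinitySections, that contains portals as child actors.
; After the parent construction script runs, it counts all instances of its own class and writes that count minus one to PortalNum on two child BP_Portal actors, one held by BPPortalOneTime.
; Both portals thus share a number derived from the instance count; the event graph holds no active logic.
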(event EventBeginPlay)

(event Collision|EventActorBeginOverlap
  (params (OtherActor :type Actor%20Object%20Reference)))

(event EventTick
  (params (DeltaSeconds :type Float%20%28single-precision%29)))

(fn ConstructionScript
  (|CallParentFunction)
  (bind _outactors (Actor|GetAllActorsOfClass "BP_EasySection7_C"))
  (Variables|/Game/Blueprints/LevelStuff/BP_Portal.BP_Portal_C|SetPortalNum (.AsBP%20Portal (Utilities|Casting|CastToBP_Portal (Variables|/Script/Engine.ChildActorComponent|GetChildActor (Variables|Default|GetBP_Portal_OneTime)))) (- (Utilities|Array|Length _outactors) 1))
  (Variables|/Game/Blueprints/LevelStuff/BP_Portal.BP_Portal_C|SetPortalNum (.AsBP%20Portal (Utilities|Casting|CastToBP_Portal (Variables|/Script/Engine.ChildActorComponent|GetChildActor (Variables|Default|GetChildActor)))) (- (Utilities|Array|Length _outactors) 1)))