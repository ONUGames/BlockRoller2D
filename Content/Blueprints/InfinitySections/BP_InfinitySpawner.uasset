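; BP_InfinitySpawner builds an endless vertical climb by stacking random sections picked for the current difficulty.
; Each NewSector call spawns a section higher up, advances difficulty at distance thresholds (wrapping after five levels), and destroys the oldest to cap the live count.
; BeginPlay logs an attempt for the starting difficulty in the global save.
; A delayed Tick check raises BPEnder behind the character, never lowering it.
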(event EventTick
  (params (DeltaSeconds :type Float%20%28single-precision%29))
  (bind _character (Variables|Default|GetCharacter))
  (bind _bp_ender (Variables|Default|GetBP_Ender))
  (bind _returnvalue (Transformation|GetActorLocation _character))
  (bind _returnvalue_2 (Transformation|GetWorldLocation _bp_ender))
  (bind (_x _y _z) (Math|Vector|BreakVector _returnvalue_2))
  (bind _z_2 (Math|Vector|BreakVector _returnvalue))
  (bind _returnvalue_3 (- _z_2 2e+03))
  (Utilities|FlowControl|Delay 2.0)
  (if (> _returnvalue_3 _z)
    (Transformation|SetWorldLocation (Variables|Default|GetBP_Ender) (Math|Vector|MakeVector _x _y _returnvalue_3) false false)))

(event EventBeginPlay
  (bind _outactors (Actor|GetAllActorsOfClass "/Game/Blueprints/Characters/BP_Character_Main.BP_Character_Main_C"))
  (Variables|Default|SetCharacter (Utilities|Array|Get(acopy) _outactors))
  (Variables|Default|SetNewVar_0 (+ (/ (Variables|/Game/Blueprints/Characters/BP_Character_Main.BP_Character_Main_C|GetCurrentDistance (Variables|Default|GetCharacter)) 1e+04) 1.0))
  (bind _output_get (Variables|Default|SetMode (Variables|Default|GetDifficulty)))
  (bind _asbp_global_save (CallFunction|GetGlobalSave))
  (switch Utilities|FlowControl|Switch|SwitchonE_Difficulties _output_get
    (:NewEnumerator0
      (Math|Integer|IncrementInt (Variables|/Game/Blueprints/BP_GlobalSave.BP_GlobalSave_C|GetTrys%20Easy _asbp_global_save)
        (:%20%20
          _)))
    (:NewEnumerator1
      (Math|Integer|IncrementInt (Variables|/Game/Blueprints/BP_GlobalSave.BP_GlobalSave_C|GetTrys%20Normal _asbp_global_save)
        (:%20%20
          _)))
    (:NewEnumerator2
      (Math|Integer|IncrementInt (Variables|/Game/Blueprints/BP_GlobalSave.BP_GlobalSave_C|GetTrys%20Hard _asbp_global_save)
        (:%20%20
          _)))
    (:NewEnumerator3
      (Math|Integer|IncrementInt (Variables|/Game/Blueprints/BP_GlobalSave.BP_GlobalSave_C|GetTrys%20Extreme _asbp_global_save)
        (:%20%20
          _)))
    (:NewEnumerator4
      (Math|Integer|IncrementInt (Variables|/Game/Blueprints/BP_GlobalSave.BP_GlobalSave_C|GetTrys%20Demonic _asbp_global_save)
        (:%20%20
          _))))
  (CallFunction|SaveGlobal _asbp_global_save))

(fn ConstructionScript)

(fn NewSector
  (bind _now (Variables|Default|GetNow))
  (bind _sectors (Variables|Default|GetSectors))
  (Utilities|FlowControl|Sequence
    (:then_0
      (bind _character (Variables|Default|GetCharacter)
        (:then
          (if (<= (Variables|Default|GetNewVar_0) (/ (Variables|/Game/Blueprints/Characters/BP_Character_Main.BP_Character_Main_C|GetCurrentDistance _character) 1e+05))
            (Variables|Default|SetDifficulty (Utilities|Enum|ByteToEnumE_Difficulties (Class|KismetMathLibrary|PercentByteByte (+ (Variables|Default|GetDifficulty) 1) 5)))
            (Variables|Default|SetNewVar_0 (+ (/ (Variables|/Game/Blueprints/Characters/BP_Character_Main.BP_Character_Main_C|GetCurrentDistance _character) 1e+05) 1.0))))
        (:else)))
    (:then_1
      (bind _output (CallFunction|GetRandomSection 0 (Variables|Default|GetDifficulty)))
      (Math|Integer|IncrementInt _now
        (:%20%20
          (bind _returnvalue (Game|SpawnActorfromClass _output (Math|Transform|MakeTransform (Math|Vector|MakeVector 0.0 0.0 (- (* _now 2e+03) 1e+02))) "Undefined" self 0))
          (Utilities|Array|Add _sectors _returnvalue)
          (if (>= (Utilities|Array|Length _sectors) 10)
            (CallFunction|DeleteOld (Utilities|Array|Get(acopy) _sectors))))))))

(fn DeleteOld
  (params (Section :type BP%20Standart%20Section%20Object%20Reference))
  (Utilities|Array|RemoveItem (Variables|Default|GetSectors) Section)
  (Actor|DestroyActor Section))