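; BP_HardSection9 is a hard-difficulty infinity section containing a key and five locked doors as child actors.
; The construction script runs the parent's script, then counts all actors of its own class in the world.
; It writes that count minus one into Num on the key and every door, giving them a shared ID based on the instance count.
; BeginPlay is empty.
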(event EventBeginPlay)

(fn ConstructionScript
  (|CallParentFunction)
  (bind _outactors (Actor|GetAllActorsOfClass (Utilities|GetClass self)))
  (Variables|/Game/Blueprints/Interactables/BP_Key.BP_Key_C|SetNum (.AsBP%20Key (Utilities|Casting|CastToBP_Key (Variables|/Script/Engine.ChildActorComponent|GetChildActor (Variables|Default|GetBP_Key)))) (- (Utilities|Array|Length _outactors) 1))
  (Variables|/Game/Blueprints/LevelStuff/BP_LockedDoor.BP_LockedDoor_C|SetNum (.AsBP%20Locked%20Door (Utilities|Casting|CastToBP_LockedDoor (Variables|/Script/Engine.ChildActorComponent|GetChildActor (Variables|Default|GetBP_LockedDoor)))) (- (Utilities|Array|Length _outactors) 1))
  (Variables|/Game/Blueprints/LevelStuff/BP_LockedDoor.BP_LockedDoor_C|SetNum (.AsBP%20Locked%20Door (Utilities|Casting|CastToBP_LockedDoor (Variables|/Script/Engine.ChildActorComponent|GetChildActor (Variables|Default|GetChildActor1)))) (- (Utilities|Array|Length _outactors) 1))
  (Variables|/Game/Blueprints/LevelStuff/BP_LockedDoor.BP_LockedDoor_C|SetNum (.AsBP%20Locked%20Door (Utilities|Casting|CastToBP_LockedDoor (Variables|/Script/Engine.ChildActorComponent|GetChildActor (Variables|Default|GetChildActor)))) (- (Utilities|Array|Length _outactors) 1))
  (Variables|/Game/Blueprints/LevelStuff/BP_LockedDoor.BP_LockedDoor_C|SetNum (.AsBP%20Locked%20Door (Utilities|Casting|CastToBP_LockedDoor (Variables|/Script/Engine.ChildActorComponent|GetChildActor (Variables|Default|GetChildActor2)))) (- (Utilities|Array|Length _outactors) 1))
  (Variables|/Game/Blueprints/LevelStuff/BP_LockedDoor.BP_LockedDoor_C|SetNum (.AsBP%20Locked%20Door (Utilities|Casting|CastToBP_LockedDoor (Variables|/Script/Engine.ChildActorComponent|GetChildActor (Variables|Default|GetChildActor3)))) (- (Utilities|Array|Length _outactors) 1)))